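; Resource deposit barrel that adds gathered resources to a team's total in the game state.
; Chunks overlapping its sphere credit the barrel's team, or the last owner's team if unassigned, then are destroyed.
; Deposit runs through ServerDeposit and MCDeposit, crediting the player's team and clearing their held item.
; Both paths trigger team-specific Niagara and sound feedback, and custom depth outlines the barrel for carrying players.
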(event `self.Sphere.OnComponentBeginOverlap`
  (params (OverlappedComponent :type "PrimitiveComponent Object Reference") (OtherActor :type "Actor Object Reference") (OtherComp :type "PrimitiveComponent Object Reference") (OtherBodyIndex :type Integer) (bFromSweep :type Boolean) (SweepResult :type "HitResult Structure (by ref)"))
  ;[1 1 1] On begin overlap with resource chunks
  (bind _asbp_base_resource_chunk (cast `/Game/Racketeers/Blueprints/GatherableItems/BP_BaseResourceChunk` OtherActor))
  (bind _asbp_player (cast `/Game/Racketeers/Core/BP_Player` (`BaseResourceChunk.LastOwner` _asbp_base_resource_chunk))
    (:`then`
      (bind _asbp_player_state (cast `/Game/Racketeers/Characters/Blueprints/BP_PlayerState` (`Pawn.PlayerState` _asbp_player))
        (:`then`
          (bind _asracketeers_game_state_base (cast `RacketeersGameStateBase` (`GameplayStatics.GetGameState`)))
          (bind (_playerinfo_playercontroller _playerinfo_playername _playerinfo_bisready _playerinfo_playerstate _playerinfo_team) (break `PlayerInfo` (`PS_Base.PlayerInfo` _asbp_player_state)))
          (`KismetSystemLibrary.PrintString` (`|GetEnumeratorNameAsString` _playerinfo_team))
          (switch `ETeams` "TeamRaccoon"
            (:`TeamRaccoon`
              (bind _value (`BaseResourceChunk.value` _asbp_base_resource_chunk))
              (bind _type (`BaseResourceChunk.type` _asbp_base_resource_chunk))
              (`RacketeersGameStateBase.AddResource` _asracketeers_game_state_base _value _type (`self.Team`) :!label _label))
            (:`TeamPanda`
              (goto _label))
            (:`NONE`
              (`RacketeersGameStateBase.AddResource` _asracketeers_game_state_base _value _type _playerinfo_team)))
          (`KismetSystemLibrary.PrintString` (`|GetEnumeratorNameAsString` _playerinfo_team))
          (`self.K2_DestroyActor` OtherActor)
          (`self.OnDepositServer` _playerinfo_team))
        (:`CastFailed`
          (`KismetSystemLibrary.PrintString` "Null playerstate"))))
    (:`CastFailed`
      (`KismetSystemLibrary.PrintString` "Null Lastplayer ref"))))

(event `OnDepositSFX`
  (params (Team :type "ETeams Enum" :default "Team_Raccoon"))
  ;[1 1 1] On deposit SFX
  (switch `ETeams` Team
    (:`TeamRaccoon`
      (`NiagaraFunctionLibrary.SpawnSystemAtLocation` "/Game/Racketeers/Art/Niagara/Deposit/FXS_Score_Stars_Raccoons.FXS_Score_Stars_Raccoons" (`SceneComponent.K2_GetComponentLocation` (`self.SFX_pointLocation`)) (struct) (1.0 1.0 1.0) true true "AutoRelease"))
    (:`TeamPanda`
      (`NiagaraFunctionLibrary.SpawnSystemAtLocation` "/Game/Racketeers/Art/Niagara/Deposit/FXS_Score_Stars_Pandas.FXS_Score_Stars_Pandas" (`SceneComponent.K2_GetComponentLocation` (`self.SFX_pointLocation`)) (struct) (1.0 1.0 1.0) true true "AutoRelease"))
    (:`NONE`
      (`NiagaraFunctionLibrary.SpawnSystemAtLocation` "/Game/Racketeers/Art/Niagara/FXS_SmokeCloud.FXS_SmokeCloud" (`SceneComponent.K2_GetComponentLocation` (`self.SFX_pointLocation`)) (struct) (1.0 1.0 1.0) true true "AutoRelease")))
  (`GameplayStatics.SpawnSoundAtLocation` "/Game/Racketeers/Audio/SFX/Environment/SFX_MaterialDeposited.SFX_MaterialDeposited" (0.0 0.0 0.0) (struct) 1.0 1.0 0.0 null null))

(event `OnDepositServer`
  (params (TeamID :type "ETeams Enum" :default "Team_Raccoon"))
  ;[1 1 1] On deposit SFX
  (`self.OnDepositSFX` TeamID))

(event `self.Deposit`
  (params (Instigator :type "Actor Object Reference"))
  ;[1 1 1] On deposit SFX
  (`self.ServerDeposit` Instigator))

(event `ServerDeposit`
  (params (Instigator :type "Actor Object Reference"))
  (`self.MCDeposit` Instigator))

(event `MCDeposit`
  (params (Instigator :type "Actor Object Reference"))
  (bind _asbp_player (cast `/Game/Racketeers/Core/BP_Player` Instigator))
  (bind (_holdingresourceinfo_resource _holdingresourceinfo_amount) (break `/Game/Racketeers/Blueprints/CraftingSystem/FCraftableResource` (`/Game/Racketeers/Core/BP_Player.HoldingResourceInfo` _asbp_player)))
  (if (`|EnumInequality` _holdingresourceinfo_resource "NONE")
    (`|ExecutionSequence`
      (:`then_0`
        (bind _asbp_player_state (cast `/Game/Racketeers/Characters/Blueprints/BP_PlayerState` (`Pawn.PlayerState` _asbp_player)))
        (bind (_playerinfo_playercontroller _playerinfo_playername _playerinfo_bisready _playerinfo_playerstate _playerinfo_team) (break `PlayerInfo` (`PS_Base.PlayerInfo` _asbp_player_state)))
        (`KismetSystemLibrary.PrintString` (`|GetEnumeratorNameAsString` _playerinfo_team))
        (bind _asbp_base_game_state (cast `/Game/Racketeers/Core/Framework/BP_BaseGameState` (`GameplayStatics.GetGameState`)))
        (`RacketeersGameStateBase.AddResource` _asbp_base_game_state _holdingresourceinfo_amount _holdingresourceinfo_resource _playerinfo_team)
        (`self.OnDepositServer` _playerinfo_team))
      (:`then_1`
        (set `/Game/Racketeers/Core/BP_Player.IsHoldingResource` false _asbp_player)
        (set `/Game/Racketeers/Core/BP_Player.HoldingResourceInfo` (make `/Game/Racketeers/Blueprints/CraftingSystem/FCraftableResource` "NONE") _asbp_player)
        (set `/Game/Racketeers/Core/BP_Player.CanChargeThrow` false _asbp_player)
        (`StaticMeshComponent.SetStaticMesh` (`/Game/Racketeers/Core/BP_Player.HoldingObject` _asbp_player) null)
        (`ActorComponent.Deactivate` (`/Game/Racketeers/Core/BP_Player.Sparkle_Effect` _asbp_player))))))

(event `Interact`
  (params (Instigator :type "Actor Object Reference")))

(event `self.ShowDepositOutline`
  (params (Instigator :type "Actor Object Reference"))
  (bind _asbp_player (cast `/Game/Racketeers/Core/BP_Player` Instigator))
  (if (`/Game/Racketeers/Core/BP_Player.IsHoldingResource` _asbp_player)
    (`PrimitiveComponent.SetRenderCustomDepth` (`self.Barrel`) true)
    (`PrimitiveComponent.SetRenderCustomDepth` (`self.Barrel1`) true)
    (`PrimitiveComponent.SetRenderCustomDepth` (`self.Barrel2`) true)
    (else
      (`PrimitiveComponent.SetRenderCustomDepth` (`self.Barrel`) false :!label _label_2)
      (`PrimitiveComponent.SetRenderCustomDepth` (`self.Barrel1`) false)
      (`PrimitiveComponent.SetRenderCustomDepth` (`self.Barrel2`) false))))

(event `self.HideDepositOutline`
  (params (Instigator :type "Actor Object Reference"))
  (goto _label_2))

(event `self.Withdraw`
  (params (Instigator :type "Actor Object Reference")))

(fn `CanInteract`
  (returns (ReturnValue :type Boolean))
  (return false))

(fn `UserConstructionScript`)
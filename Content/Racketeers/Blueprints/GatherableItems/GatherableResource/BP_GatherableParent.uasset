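; Base Blueprint for gatherable resources that players hit through InteractInterface until they break and drop loot.
; Each hit lowers ResourceHP and multicasts a scale animation, traced impact FX with sound, and a health widget update, which OnRep_ResourceHP also refreshes.
; At zero HP, it spawns loot launched upward in a random cone after a short delay, then destroys itself.
; InteractionArea overlaps toggle a custom depth highlight for the local player only.
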(event `self.ReceiveBeginPlay`
  (bind _aswbp_gatherable_health (cast `/Game/Racketeers/Blueprints/Widgets/WBP_GatherableHealth` (`WidgetComponent.GetUserWidgetObject` (`self.Health`))))
  (`/Game/Racketeers/Blueprints/Widgets/WBP_GatherableHealth.Init` _aswbp_gatherable_health self (`self.ResourceHP`)))

(event `self.ReceiveTick`
  (params (DeltaSeconds :type "Float (single-precision)")))

(event `self.StartInteract`
  (params (Instigator :type "Actor Object Reference") (bIsServer :type Boolean))
  ;[1 1 1] InteractInterface
  (`KismetSystemLibrary.PrintString` "InteractGatherable")
  (`self.ApplyGatheringdamage` Instigator)
  (`self.ServerOnHitUI` self))

(event `SpawnOnServer`
  ;[1 1 1] SpawnLoot on server
  (`KismetSystemLibrary.Delay` 0.2)
  (`self.SpawnLoot`)
  (`self.K2_DestroyActor`))

(event `OnHitAnimation`
  (params (Instigator :type "/Game/Racketeers/Blueprints/GatherableItems/GatherableResource/BP_GatherableParent Object Reference"))
  ;[1 1 1] On hit animation
  (`self.MultiCastHitAnimation` Instigator))

(event `MultiCastHitAnimation`
  (params (Instigator :type "/Game/Racketeers/Blueprints/GatherableItems/GatherableResource/BP_GatherableParent Object Reference"))
  ;[1 1 1] On hit animation
  ;;[1 0.03922 0] MultiCast Hit Animation
  (bind (_direction _scaletrack) (`Timeline|Timeline` :!via `PlayFromStart`)
    (:`Update`
      (`SceneComponent.SetWorldScale3D` (`/Game/Racketeers/Blueprints/GatherableItems/GatherableResource/BP_GatherableParent.StaticMesh` Instigator) (`KismetMathLibrary.Conv_DoubleToVector` _scaletrack)))))

(event `OnHitFXS`
  (params (Instigator :type "/Game/Racketeers/Blueprints/GatherableItems/GatherableResource/BP_GatherableParent Object Reference") (ActorPlayer :type "Actor Object Reference"))
  ;[1 1 1] On Hit FXS
  (`self.MultiCastHitFXS` Instigator ActorPlayer))

(event `MultiCastHitFXS`
  (params (Instigator :type "/Game/Racketeers/Blueprints/GatherableItems/GatherableResource/BP_GatherableParent Object Reference") (ActorPlayer :type "Actor Object Reference"))
  ;[1 1 1] On Hit FXS
  ;;[1 0.03922 0] MultiCast On Hit FXS
  (bind _outhit (`KismetSystemLibrary.LineTraceSingleForObjects` (`SceneComponent.K2_GetComponentLocation` (`self.GetComponentByClass` ActorPlayer "/Script/Engine.SpringArmComponent")) (`SceneComponent.K2_GetComponentLocation` (`/Game/Racketeers/Blueprints/GatherableItems/GatherableResource/BP_GatherableParent.GatherPoint` Instigator)) (`self.Object Types`) false (`|MakeArray` ActorPlayer) "None" false (struct :`R` 1.0 :`G` 0.916018 :`B` 0.957652 :`A` 1.0) (struct :`G` 0.109944 :`B` 1.0 :`A` 1.0)))
  (bind (_bblockinghit _binitialoverlap _time _distance _location _impactpoint) (`GameplayStatics.BreakHitResult` _outhit))
  (`NiagaraFunctionLibrary.SpawnSystemAtLocation` (`/Game/Racketeers/Blueprints/GatherableItems/GatherableResource/BP_GatherableParent.OnHit_FXS` Instigator) _impactpoint (struct) (1.0 1.0 1.0) true true "AutoRelease")
  (`GameplayStatics.PlaySoundAtLocation` (`self.Sound`) _impactpoint (struct) 1.0 1.0 0.0 null null null null))

(event `ServerOnHitUI`
  (params (Instigator :type "/Game/Racketeers/Blueprints/GatherableItems/GatherableResource/BP_GatherableParent Object Reference"))
  ;[1 1 1] Server On Hit UI
  (`self.MultiCastOnHitUI` Instigator))

(event `MultiCastOnHitUI`
  (params (Instigator :type "/Game/Racketeers/Blueprints/GatherableItems/GatherableResource/BP_GatherableParent Object Reference"))
  ;[1 1 1] Server On Hit UI
  ;;[1 0.03922 0] Multi Cast On Hit UI
  (bind _aswbp_gatherable_health (cast `/Game/Racketeers/Blueprints/Widgets/WBP_GatherableHealth` (`WidgetComponent.GetUserWidgetObject` (`/Game/Racketeers/Blueprints/GatherableItems/GatherableResource/BP_GatherableParent.Health` Instigator))))
  (`/Game/Racketeers/Blueprints/Widgets/WBP_GatherableHealth.Update` _aswbp_gatherable_health))

(event `self.Interaction Area.OnComponentBeginOverlap`
  (params (OverlappedComponent :type "PrimitiveComponent Object Reference") (OtherActor :type "Actor Object Reference") (OtherComp :type "PrimitiveComponent Object Reference") (OtherBodyIndex :type Integer) (bFromSweep :type Boolean) (SweepResult :type "HitResult Structure (by ref)"))
  (if (`Pawn.IsLocallyControlled` (`Actor.Instigator` OtherActor))
    (`PrimitiveComponent.SetRenderCustomDepth` (`self.StaticMesh`) true)))

(event `self.Interaction Area.OnComponentEndOverlap`
  (params (OverlappedComponent :type "PrimitiveComponent Object Reference") (OtherActor :type "Actor Object Reference") (OtherComp :type "PrimitiveComponent Object Reference") (OtherBodyIndex :type Integer))
  (if (`Pawn.IsLocallyControlled` (`Actor.Instigator` OtherActor))
    (`PrimitiveComponent.SetRenderCustomDepth` (`self.StaticMesh`) false)))

(fn `ApplyGatheringdamage`
  (params (Instigator :type "Actor Object Reference"))
  ;[1 1 1] Apply damaged to the object
  (`self.OnHitFXS` self Instigator)
  (`self.OnHitAnimation` self)
  (bind _output_get (set `self.ResourceHP` (- (`self.ResourceHP`) (`self.InitialGatheringDamage`))))
  (if (<= _output_get 0.0)
    (`self.SpawnOnServer`)))

(fn `CanInteract`
  (returns (ReturnValue :type Boolean))
  ;[1 1 1] CanInteract
  (if (> (`self.ResourceHP`) 0.0)
    (return true)
    (else
      (return false))))

(fn `GenerateRandomLocation`
  (returns (LocationToSpawn :type "Vector Structure"))
  ;[1 1 1] Generates random locations close to a specific point
  (return (+ (`SceneComponent.K2_GetComponentLocation` (`self.StaticMesh`)) (* (`KismetMathLibrary.GreaterGreater_VectorRotator` (1.0 0.0 0.0) (`KismetMathLibrary.MakeRotator` 0.0 0.0 (`KismetMathLibrary.RandomFloatInRange` 0.0 360.0))) (`KismetMathLibrary.RandomFloatInRange` (* (`self.LootSpawnMaxDistance`) -1.0) (`self.LootSpawnMaxDistance`))))))

(fn `OnRep_ResourceHP`
  (bind _aswbp_gatherable_health (cast `/Game/Racketeers/Blueprints/Widgets/WBP_GatherableHealth` (`WidgetComponent.GetUserWidgetObject` (`self.Health`))))
  (`/Game/Racketeers/Blueprints/Widgets/WBP_GatherableHealth.Update` _aswbp_gatherable_health))

(fn `SpawnLoot`
  ;[1 1 1] Spawns loot near to the parent object
  (`PrimitiveComponent.SetCollisionEnabled` (`self.StaticMesh`) "NoCollision")
  (for _ (range 1 (+ (`self.AmountLootToSpawn`) 1))
    (bind _returnvalue (`|SpawnActorFromClass` (`self.LootToSpawn`) (`KismetMathLibrary.Conv_VectorToTransform` (`self.K2_GetActorLocation`)) "Undefined" "MultiplyWithRoot" null (0.0 0.0 1.0) 500.0 null))
    (`PrimitiveComponent.AddImpulse` (`BaseResourceChunk.ResourceMesh` _returnvalue) (* (`KismetMathLibrary.RandomFloatInRange` 500.0 1000.0) (`KismetMathLibrary.RandomUnitVectorInConeInDegrees` (0.0 0.0 1.0) 45.0)) "None" false)))

(fn `UserConstructionScript`)
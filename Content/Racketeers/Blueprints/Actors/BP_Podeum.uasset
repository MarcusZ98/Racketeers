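; BP_Podeum is a podium actor that appears to be a claimable spot for a player identified by team and team player ID.
; CheckAvalability returns false if the podium is taken; otherwise it marks it taken, then returns the team and ID comparison, so even a failed match claims it.
; SpawnPawn, OnWinner, OnLoser, BeginPlay and the construction script are empty here.
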(event `SpawnPawn`
  (params (PC :type "PlayerController Object Reference")))

(event `OnWinner`)

(event `self.ReceiveBeginPlay`)

(event `OnLoser`)

(fn `CheckAvalability`
  (params (Team :type "ETeams Enum" :default "Team_Raccoon") (TeamPlayerID :type Integer))
  (returns (Avalible :type Boolean))
  (if (`self.Taken`)
    (return false)
    (else
      (set `self.Taken` true)
      (return (and (== (`KismetSystemLibrary.MakeLiteralByte` (`self.Team`)) Team) (== (`self.TeamPlayerID`) TeamPlayerID))))))

(fn `UserConstructionScript`)
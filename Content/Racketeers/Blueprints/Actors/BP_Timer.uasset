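; BP_Timer is a timer actor that shows a timer widget to the player.
; SetWidget adds TimerWidget to player 0's viewport, links it back to this actor and calls SetServerTimeSeconds on the RacketeersController with a zeroed, inactive state.
; BeginPlay starts a looping one-second event timer and caches its handle.
; An authority-checked multicast activation remains in the graph but is disconnected.
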(event `SetWidget`
  (bind _returnvalue (`GameplayStatics.GetPlayerController` 0))
  (bind _timer_widget (`self.Timer Widget`))
  (bind _asbp_player_controller (cast `/Game/Racketeers/Characters/Blueprints/PCs/BP_PlayerController` _returnvalue))
  (`KismetSystemLibrary.PrintString` (`AdvancedSessionsLibrary.UniqueNetIdToString` (`AdvancedSessionsLibrary.GetUniqueNetID` (`GameplayStatics.GetPlayerController` 0))))
  (`RacketeersController.AddWidgetToViewport` _asbp_player_controller _timer_widget)
  (bind _aswbp_timer (cast `/Game/Racketeers/Blueprints/Widgets/WBP_Timer` _timer_widget))
  (set `/Game/Racketeers/Blueprints/Widgets/WBP_Timer.Timer` self _aswbp_timer)
  (bind _asracketeers_controller (cast `RacketeersController` _returnvalue))
  (`RacketeersController.SetServerTimeSeconds` _asracketeers_controller _asracketeers_controller 0.0 false))

(event `self.ReceiveBeginPlay`
  (bind _returnvalue (`KismetSystemLibrary.K2_SetTimerDelegate` (`|CreateDelegate` :!event `SetWidget `) 1.0 true))
  (set `self.CachHandle` _returnvalue))

(event `self.ReceiveTick`
  (params (DeltaSeconds :type "Float (single-precision)")))

(fn `UserConstructionScript`)
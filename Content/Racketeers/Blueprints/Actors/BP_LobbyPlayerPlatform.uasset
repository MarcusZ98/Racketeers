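; BP_LobbyPlayerPlatform is a lobby slot that displays a player's team character and offers a friend-list button while empty.
; SpawnCharacter splits players into Panda and Raccoon halves by index, passes team and ID to the lobby PlayerController, and spawns the matching character.
; On the server, the button links to one BP_FriendList actor, which moves to whichever platform opens it.
; MakeUnique colors the platform by team ID; Clear empties the slot.
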(event `self.ReceiveBeginPlay`
  (`self.SetUpServer`))

(event `SpawnCharacter`
  (params (PC :type "PlayerController Object Reference") (Index :type Integer))
  (bind _asbp_lobby_pc (cast `/Game/Racketeers/Characters/Blueprints/PCs/BP_LobbyPC` (`self.PC`) :!pure true))
  (bind _returnvalue (/ (`self.NumberOfPlayers`) 2))
  (bind _returnvalue_2 (- _returnvalue 1))
  (bind _returnvalue_3 (select `bool` (`KismetMathLibrary.InRange_IntInt` Index 0 _returnvalue_2) :`false` "TeamRaccoon" :`true` "TeamPanda" :!type "ETeams Enum"))
  (set `self.PC` PC)
  (bind _currentcharacter (`self.CurrentCharacter`)
    (:`then`
      (`self.K2_DestroyActor` _currentcharacter))
    (:`else`
      _))
  (bind _structout (setmembers `PlayerInfo` :`StructRef` (`/Game/Racketeers/Characters/Blueprints/PCs/BP_LobbyPC.PlayerInfoPC` _asbp_lobby_pc) :`Team` _returnvalue_3 :`TeamPlayerID` (`KismetMathLibrary.SelectInt` (- Index _returnvalue) Index (> Index _returnvalue_2))))
  (bind (_playercontroller _playername _bisready _playerstate _team _teamplayerid) (break `PlayerInfo` _structout))
  (`/Game/Racketeers/Characters/Blueprints/PCs/BP_LobbyPC.SetUpPlatform` _asbp_lobby_pc self _teamplayerid _team)
  (bind _returnvalue_4 (`|SpawnActorFromClass` (select `ETeams` _returnvalue_3 :!type "Actor Class Reference") (`SceneComponent.K2_GetComponentToWorld` (`self.PlayerSpawnTransform`)) "Undefined" "MultiplyWithRoot" null null))
  (set `self.CurrentCharacter` _returnvalue_4)
  (`SceneComponent.SetVisibility` (`self.OpenFriendListButton`) false false)
  (if (== (`SceneComponent.K2_GetComponentLocation` (`self.FriendListLocation`)) (`self.K2_GetActorLocation` (`self.FriendListREF`)) :`ErrorTolerance` 2.0)
    (`/Game/Racketeers/Blueprints/Actors/BP_FriendList.Show` (`self.FriendListREF`) false null)))

(event `Clear`
  (set `self.PC` null)
  (bind _currentcharacter (`self.CurrentCharacter`)
    (:`then`
      (`self.K2_DestroyActor` _currentcharacter)
      (set `self.CurrentCharacter` null))
    (:`else`
      _))
  (`SceneComponent.SetVisibility` (`self.OpenFriendListButton`) true false))

(fn `MakeUnique`
  (params (TeamID :type Integer) (Team :type "ETeams Enum" :default "Team_Raccoon"))
  (switch `int` TeamID
    (:`0`
      (`PrimitiveComponent.SetMaterial` (`self.Platform`) 0 "/AnimationSharing/AnimSharingBlue.AnimSharingBlue"))
    (:`1`
      (`PrimitiveComponent.SetMaterial` (`self.Platform`) 0 "/AnimationSharing/AnimSharingGreen.AnimSharingGreen"))
    (:`2`
      (`PrimitiveComponent.SetMaterial` (`self.Platform`) 0 "/AnimationSharing/AnimSharingRed.AnimSharingRed"))))

(fn `SetUpServer`
  (if (`KismetSystemLibrary.IsServer`)
    (bind _returnvalue (`GameplayStatics.GetActorOfClass` "/Game/Racketeers/Blueprints/Actors/BP_FriendList.BP_FriendList_C"))
    (set `self.FriendListREF` _returnvalue)
    (bind _aswbp_open_friend_list_button (cast `/Game/Racketeers/Blueprints/Widgets/WBP_OpenFriendListButton` (`WidgetComponent.GetWidget` (`self.OpenFriendListButton`))))
    (set `/Game/Racketeers/Blueprints/Widgets/WBP_OpenFriendListButton.LobbyPlayerPlatformREF` self _aswbp_open_friend_list_button)
    (`SceneComponent.SetVisibility` (`self.OpenFriendListButton`) true false)))

(fn `ShowFriendList`
  (params (bShow :type Boolean))
  (bind _returnvalue (`WidgetComponent.GetWidget` (`self.OpenFriendListButton`)))
  (if bShow
    (`Widget.SetVisibility` _returnvalue "Collapsed")
    (`self.K2_SetActorLocation` (`self.FriendListREF`) (`SceneComponent.K2_GetComponentLocation` (`self.FriendListLocation`)) false false)
    (`/Game/Racketeers/Blueprints/Actors/BP_FriendList.Show` (`self.FriendListREF`) true self)
    (else
      (`Widget.SetVisibility` _returnvalue "Visible"))))

(fn `UserConstructionScript`)
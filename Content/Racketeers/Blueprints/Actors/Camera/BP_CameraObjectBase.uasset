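; Shared camera actor that follows the center of all player actors and can tether stragglers to the group.
; Each tick it interpolates toward their averaged ground position plus an offset, scaling spring arm length with the farthest player's distance, within clamped limits.
; When tethering is enabled, players beyond the maximum horizontal distance are moved to their KnockbackPosition component, both directly and through a server set-location event.
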(event `Server_SetLocation`
  (params (Location :type "Vector Structure") (Actor :type "Actor Object Reference"))
  ;[1 1 1] Tethering
  (`self.K2_SetActorLocation` Actor Location false false))

(event `self.ReceiveBeginPlay`
  (bind _asbp_player (cast `/Game/Racketeers/Core/BP_Player` (`GameplayStatics.GetPlayerPawn` 0)))
  (bind _output_get (set `self.Player` _asbp_player))
  (bind _asbp_player_state (cast `/Game/Racketeers/Characters/Blueprints/BP_PlayerState` (`Pawn.PlayerState` _output_get)))
  (set `self.PlayerState` _asbp_player_state))

(event `self.ReceiveTick`
  (params (DeltaSeconds :type "Float (single-precision)"))
  (bind (_returnvalue_x _returnvalue_y) (`KismetMathLibrary.BreakVector` (`self.K2_GetActorLocation`)))
  (bind _outactors (`GameplayStatics.GetAllActorsOfClass` (`self.Player Class`)))
  (for _array_element _outactors
    (bind (_returnvalue_x_2 _returnvalue_y_2 _returnvalue_z) (`KismetMathLibrary.BreakVector` (`self.K2_GetActorLocation` _array_element)))
    (set `self.Position` (+ (`KismetMathLibrary.MakeVector` _returnvalue_x_2 _returnvalue_y_2) (`self.Position`))))
  (bind _returnvalue (`KismetArrayLibrary.Array_Length` _outactors))
  (if (> _returnvalue 0)
    (`self.K2_SetActorLocation` (`KismetMathLibrary.VInterpTo` (`self.K2_GetActorLocation`) (+ (/ (`self.Position`) _returnvalue) (`self.Offset`)) DeltaSeconds 2.6))
    (for _array_element_2 _outactors
      (`|ExecutionSequence`
        (:`then_0`
          (bind (_returnvalue_x_3 _returnvalue_y_3) (`KismetMathLibrary.BreakVector` (`self.K2_GetActorLocation` _array_element_2)))
          (bind _returnvalue_2 (`KismetMathLibrary.Vector_Distance` (`KismetMathLibrary.MakeVector` _returnvalue_x_3 _returnvalue_y_3) (`KismetMathLibrary.MakeVector` _returnvalue_x _returnvalue_y)))
          ;[1 1 1] Tethering
          (if (and (>= _returnvalue_2 (`self.MaxDistanceForPlayers`)) (`self.ShouldTether`))
            (bind _returnvalue_3 (`SceneComponent.K2_GetComponentLocation` (`/Game/Racketeers/Core/BP_Player.KnockbackPosition` _array_element_2)))
            (`self.K2_SetActorLocation` _array_element_2 _returnvalue_3 false false)
            (`self.Server_SetLocation` _returnvalue_3 _array_element_2)))
        (:`then_1`
          (if (>= _returnvalue_2 (`self.Distance To Furthest Player`))
            (set `self.Distance To Furthest Player` _returnvalue_2)))))
    (set `SpringArmComponent.TargetArmLength` (`KismetMathLibrary.FClamp` (+ (`self.Default Zoom value`) (* (`self.Distance To Furthest Player`) (`self.Camera Zoom Multiplier`))) (`self.Min Arn Length`) (`self.Max Arm Length`)) (`self.SpringArm`))
    (set `self.Position` (0.0 0.0 100.0))
    (set `self.Distance To Furthest Player` 0.0)))

(fn `UserConstructionScript`)
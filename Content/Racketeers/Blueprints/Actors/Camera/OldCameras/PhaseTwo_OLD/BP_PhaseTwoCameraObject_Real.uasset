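; Phase two camera actor, stored under old cameras, that makes itself the view target of the first player controller.
; On Tick it caches the local BP_Player and its BP_PlayerState, then switches the view to itself whenever another target is active.
; A team-match check and a delayed BP_Racoon variant are left unconnected, so the takeover applies regardless of team.
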(event `self.ReceiveBeginPlay`)

(event `self.ReceiveTick`
  (params (DeltaSeconds :type "Float (single-precision)"))
  (bind _returnvalue (`GameplayStatics.GetPlayerController` 0))
  (`/Engine/EditorBlueprintResources/StandardMacros.IsValid` (`self.Player`)
    (:`Is Valid`
      (if (not (== (`Controller.GetViewTarget` _returnvalue) self))
        (`PlayerController.SetViewTargetWithBlend` _returnvalue self 0.0 "VTBlend_Linear" 0.0 false)))
    (:`Is Not Valid`
      (bind _asbp_player (cast `/Game/Racketeers/Core/BP_Player` (`GameplayStatics.GetPlayerPawn` 0)))
      (bind _output_get (set `self.Player` _asbp_player))
      (bind _asbp_player_state (cast `/Game/Racketeers/Characters/Blueprints/BP_PlayerState` (`Pawn.PlayerState` _output_get)))
      (set `self.PlayerState` _asbp_player_state))))

(fn `UserConstructionScript`
  (`parent.UserConstructionScript`))
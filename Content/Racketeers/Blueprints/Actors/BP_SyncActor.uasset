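; Sync actor that shows and removes a waiting-screen widget while players join a networked session.
; A server event forwards the show call to a client while a sync is in progress.
; A removal check counts valid PlayerArray entries against the expected total, then clears its timer and multicasts widget removal.
; The setup that records the expected total and starts that looping timer is disconnected, and Count is never reset between checks.
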(event `ClientAddSyncScreen`
  (params (NewParam :type "/Game/Racketeers/Blueprints/Actors/BP_SyncActor Object Reference"))
  (`UserWidget.AddToViewport` (`self.SyncWidget`) 0))

(event `ServerAddSyncScreen`
  (params (NewParam :type "/Game/Racketeers/Blueprints/Actors/BP_SyncActor Object Reference"))
  (if (`self.InProgress`)
    (`self.ClientAddSyncScreen` NewParam null)))

(event `self.ReceiveBeginPlay`)

(event `RemoveSyncScreen`
  (for _array_element (`GameStateBase.PlayerArray` (`GameplayStatics.GetGameState`))
    (`/Engine/EditorBlueprintResources/StandardMacros.IsValid` _array_element
      (:`Is Valid`
        (`/Engine/EditorBlueprintResources/StandardMacros.IncrementInt` (`self.Count`)))))
  (if (== (`self.PlayerSupposedToJoin`) (`self.Count`))
    (`KismetSystemLibrary.K2_ClearAndInvalidateTimerHandle` (`self.CacheHandle`))
    (set `self.InProgress` false)
    (`self.MultiRemoveSyncScreen`)))

(event `MultiRemoveSyncScreen`
  (`Widget.RemoveFromParent` (`self.SyncWidget`)))

(fn `UserConstructionScript`)
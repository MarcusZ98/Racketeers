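; Level transition actor that holds play until all players have joined, then reveals the game with a WBP_Transition iris-in.
; Looping timers report the local player through BP_PlayerController and, on the server, compare PlayersJoined against the PlayerArray size.
; On a match, the server resets the count, calls AllStagesFinished on the game mode and fires MultiCastRemoveScrren to play the iris.
; Without a RacketeersGameStateBase, Tick plays the iris once instead.
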(event `ClientAddSyncScreen`
  (params (NewParam :type "/Game/Racketeers/Blueprints/Actors/BP_SyncActor Object Reference"))
  (`UserWidget.AddToViewport` (`self.SyncWidget`) 0))

(event `Incremenct Count`
  (`/Engine/EditorBlueprintResources/StandardMacros.IncrementInt` (`self.Count`)))

(event `self.ReceiveTick`
  (params (DeltaSeconds :type "Float (single-precision)"))
  (bind _addedduration (`self.AddedDuration`))
  (cast `RacketeersGameStateBase` (`GameplayStatics.GetGameState`)
    (:`CastFailed`
      (`/Engine/EditorBlueprintResources/StandardMacros.DoOnce` false
        (:`Completed`
          (bind _returnvalue (`|CreateWidget` "/Game/Racketeers/Blueprints/Widgets/WBP_Transition.WBP_Transition_C"))
          (bind _output_get (set `self.SyncWidget` _returnvalue))
          (`UserWidget.AddToViewport` _returnvalue 0)
          (`UserWidget.AddToViewport` _output_get 0)
          (`/Game/Racketeers/Blueprints/Widgets/WBP_Transition.IrisIn` _returnvalue _addedduration)
          (`KismetSystemLibrary.Delay` (+ _addedduration 1.0))
          (`Widget.RemoveFromParent` _returnvalue)
          (`self.SetActorTickEnabled` false))))))

(event `PlayerJoined`
  (bind _returnvalue (`GameplayStatics.GetPlayerController` 0))
  (`KismetSystemLibrary.PrintString` "Player Joined " true true (struct :`R` 0.999918 :`G` 1.0 :`A` 1.0) 100.0)
  (`/Engine/EditorBlueprintResources/StandardMacros.IsValid` _returnvalue
    (:`Is Valid`
      (`KismetSystemLibrary.K2_ClearAndInvalidateTimerHandle` (`self.Player Joined Time Handl`))
      (bind _asbp_player_controller (cast `/Game/Racketeers/Characters/Blueprints/PCs/BP_PlayerController` _returnvalue))
      (`/Game/Racketeers/Characters/Blueprints/PCs/BP_PlayerController.incrementPlayerJoined` _asbp_player_controller))))

(event `self.ReceiveBeginPlay`
  (`KismetSystemLibrary.PrintString` (`KismetStringLibrary.Conv_IntToString` (`KismetArrayLibrary.Array_Length` (`GameStateBase.PlayerArray` (`GameplayStatics.GetGameState`)))) true true (struct :`R` 1.0 :`G` 0.80655 :`A` 1.0) 10000.0)
  (bind _returnvalue (`KismetSystemLibrary.K2_SetTimerDelegate` (`|CreateDelegate` :!event `PlayerJoined`) 0.2 true))
  (set `self.Player Joined Time Handl` _returnvalue)
  (`/Engine/EditorBlueprintResources/ActorMacros.Switch Has Authority`
    (:`Authority`
      (set `self.InProgress` true)
      (set `self.PlayerSupposedToJoin` (`KismetArrayLibrary.Array_Length` (`GameStateBase.PlayerArray` (`GameplayStatics.GetGameState`))))
      (bind _returnvalue_2 (`KismetSystemLibrary.K2_SetTimerDelegate` (`|CreateDelegate` :!event `RemoveSyncScreen`) 1.0 true))
      (set `self.CacheHandle` _returnvalue_2))))

(event `RemoveSyncScreen`
  (bind _returnvalue (`GameplayStatics.GetGameState`))
  (bind _asracketeers_game_state_base (cast `RacketeersGameStateBase` _returnvalue))
  (bind _playersjoined (`RacketeersGameStateBase.PlayersJoined` _asracketeers_game_state_base))
  (`KismetSystemLibrary.PrintString` (`KismetStringLibrary.Concat_StrStr` "EXPECTED: " (`KismetStringLibrary.Conv_IntToString` 0) " Count: " (`KismetStringLibrary.Conv_IntToString` _playersjoined)) true true (struct :`G` 1.0 :`B` 0.008223 :`A` 1.0) 1000.0)
  (if (== (`KismetArrayLibrary.Array_Length` (`GameStateBase.PlayerArray` _returnvalue)) _playersjoined)
    (`/Engine/EditorBlueprintResources/StandardMacros.IsValid` _asracketeers_game_state_base
      (:`Is Valid`
        (set `RacketeersGameStateBase.PlayersJoined` 0 _asracketeers_game_state_base)
        (`KismetSystemLibrary.K2_ClearAndInvalidateTimerHandle` (`self.CacheHandle`))
        (set `self.InProgress` false)
        (`Widget.RemoveFromParent` (`self.SyncWidget`))
        (bind _asracketeers_gmbase (cast `RacketeersGMBase` (`GameplayStatics.GetGameMode`)))
        (`RacketeersGMBase.AllStagesFinished` _asracketeers_gmbase)
        (`self.MultiCastRemoveScrren`)))))

(event `MultiCastRemoveScrren`
  (bind _addedduration (`self.AddedDuration`))
  (bind _returnvalue (`|CreateWidget` "/Game/Racketeers/Blueprints/Widgets/WBP_Transition.WBP_Transition_C"))
  (bind _output_get (set `self.SyncWidget` _returnvalue))
  (`UserWidget.AddToViewport` _returnvalue 0)
  (`UserWidget.AddToViewport` _output_get 0)
  (`/Game/Racketeers/Blueprints/Widgets/WBP_Transition.IrisIn` _returnvalue _addedduration)
  (`KismetSystemLibrary.Delay` (+ _addedduration 1.0))
  (`Widget.RemoveFromParent` _returnvalue)
  (`self.SetActorTickEnabled` false))

(fn `MultiRemoveSyncScreen`)

(fn `UserConstructionScript`)
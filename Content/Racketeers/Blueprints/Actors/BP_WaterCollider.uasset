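; BP_WaterCollider is a water hazard volume in Racketeers that stuns and respawns players who touch it.
; On box overlap, the authority respawns the player through RacketeersGMBase and triggers stun audio, splash, respawn and stun effects.
; Movement is disabled on server and multicast, then a client event stuns and slows the player, using a timer to restore walk speed cached from player 0 at BeginPlay.
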(event `ClientSLowSpeed`
  (params (NewParam :type "/Game/Racketeers/Core/BP_Player Object Reference") (NewParam2 :type "Float (double-precision)"))
  (`KismetSystemLibrary.PrintString` "Start Client Slow Down Speed")
  (set `CharacterMovementComponent.MaxWalkSpeed` 50.0 (`Character.CharacterMovement` NewParam))
  (set `/Game/Racketeers/Core/BP_Player.IsStunned` true NewParam)
  (bind _returnvalue (`KismetSystemLibrary.K2_SetTimerDelegate` (`|CreateDelegate` :!event `CustomEvent`) 2.0 true))
  (set `self.CacheTimer` _returnvalue))

(event `CustomEvent`
  (`KismetSystemLibrary.PrintString` "GIVE BACK MOVEMENT SPEED")
  (`KismetSystemLibrary.PrintString` (`AdvancedSessionsLibrary.UniqueNetIdToString` (`AdvancedSessionsLibrary.GetUniqueNetIDFromPlayerState` (`Pawn.PlayerState` (stale `ClientSLowSpeed` NewParam)))))
  (set `/Game/Racketeers/Core/BP_Player.IsStunned` false (stale `ClientSLowSpeed` NewParam))
  (set `CharacterMovementComponent.MaxWalkSpeed` (stale `ClientSLowSpeed` NewParam2) (`Character.CharacterMovement` (stale `ClientSLowSpeed` NewParam)))
  (`KismetSystemLibrary.K2_ClearAndInvalidateTimerHandle` (`self.CacheTimer`)))

(event `ServerSlowSpeed`
  (params (NewParam :type "/Game/Racketeers/Core/BP_Player Object Reference"))
  (`CharacterMovementComponent.DisableMovement` (`Character.CharacterMovement` NewParam))
  (`self.MultiCastSlowSpeed` NewParam (`self.TempWalkspeed`)))

(event `ServerHandleWaterOverlap`
  (params (Player :type "/Game/Racketeers/Core/BP_Player Object Reference") (InpactPoint :type "Vector Structure"))
  (bind _effectscomponent (`/Game/Racketeers/Core/BP_Player.EffectsComponent` Player))
  (bind _asracketeers_gmbase (cast `RacketeersGMBase` (`GameplayStatics.GetGameMode`)))
  (`self.ServerSlowSpeed` Player)
  (`RacketeersGMBase.RespawnPlayer` _asracketeers_gmbase (`Pawn.PlayerState` Player))
  (`/Game/Racketeers/Blueprints/Components/EffectsComponent.StunAudio` _effectscomponent)
  (`/Game/Racketeers/Blueprints/Components/EffectsComponent.MultiSpawnAtEffectAtPosition` _effectscomponent "/Game/Racketeers/Art/Niagara/Water/FXS_Splash.FXS_Splash" InpactPoint)
  (`/Game/Racketeers/Blueprints/Components/EffectsComponent.MultiSpawnAtEffectAtPosition` _effectscomponent "/Game/Racketeers/Art/Niagara/Player/FXS_Respawn.FXS_Respawn" (`self.K2_GetActorLocation` Player))
  (`/Game/Racketeers/Blueprints/Components/EffectsComponent.ServerOneEffectCall` _effectscomponent (`/Game/Racketeers/Core/BP_Player.PlayerStunnedEffect` Player)))

(event `MultiCastSlowSpeed`
  (params (NewParam :type "/Game/Racketeers/Core/BP_Player Object Reference") (NewParam2 :type "Float (double-precision)"))
  (`CharacterMovementComponent.DisableMovement` (`Character.CharacterMovement` NewParam))
  (`/Game/Racketeers/Core/BP_Player.ClientSLowSpeed` (stale `ServerSlowSpeed` NewParam) NewParam NewParam2)
  (`/Game/Racketeers/Core/BP_Player.ClientSLowSpeed` NewParam NewParam NewParam2))

(event `self.ReceiveBeginPlay`
  (if (`self.HasAuthority` (`GameplayStatics.GetGameState`))
    (set `self.TempWalkspeed` (`CharacterMovementComponent.MaxWalkSpeed` (`Character.CharacterMovement` (`GameplayStatics.GetPlayerCharacter` 0))))))

(event `self.Box.OnComponentBeginOverlap`
  (params (OverlappedComponent :type "PrimitiveComponent Object Reference") (OtherActor :type "Actor Object Reference") (OtherComp :type "PrimitiveComponent Object Reference") (OtherBodyIndex :type Integer) (bFromSweep :type Boolean) (SweepResult :type "HitResult Structure (by ref)"))
  (bind _asbp_player (cast `/Game/Racketeers/Core/BP_Player` OtherActor))
  (if (`self.HasAuthority` (`GameplayStatics.GetGameState`))
    (`self.ServerHandleWaterOverlap` _asbp_player SweepResult_ImpactPoint)))

(fn `UserConstructionScript`)
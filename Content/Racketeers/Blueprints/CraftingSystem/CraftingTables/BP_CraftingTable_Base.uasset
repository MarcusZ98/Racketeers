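; Base team crafting bench that turns deposited wood, fiber and metal into hull, cannon or sail upgrades.
; Players deposit by interacting or throwing chunks into a hitbox, which respawns unneeded ones as a throw-back.
; Deposits are checked against the next DT_CraftableItem row and update a world widget; completed recipes add the part to the game state.
; Setup restores upgrade stage and saved progress from the game state, and multicast events mirror thrown deposits to clients.
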(event `Set Widget`
  (`/Engine/EditorBlueprintResources/StandardMacros.IsValid` (`GameplayStatics.GetPlayerController` 0)
    (:`Is Valid`
      (`KismetSystemLibrary.K2_ClearAndInvalidateTimerHandle` (`self.Handler Player joined`))
      (`|ExecutionSequence`
        (:`then_0`
          (bind _asbp_base_game_state (cast `/Game/Racketeers/Core/Framework/BP_BaseGameState` (`GameplayStatics.GetGameState`)))
          (bind _part (`self.GetTeamPart` _asbp_base_game_state))
          (if (== _part (`|GetArrayItem` (`self.Parts`) 1))
            (`KismetArrayLibrary.Array_Clear` (`self.ListOfUpgrades`))
            (elif (== _part (`|GetArrayItem` (`self.Parts`)))
              (`KismetArrayLibrary.Array_Remove` (`self.ListOfUpgrades`)))))
        (:`then_1`
          (`self.UpdateWidget`))
        (:`then_2`
          (bind _asbp_base_game_state_2 (cast `/Game/Racketeers/Core/Framework/BP_BaseGameState` (`GameplayStatics.GetGameState`)))
          (bind _progress (`self.GetCraftingProgress` _asbp_base_game_state_2))
          (`self.GiveResources` "WOOD" (`KismetArrayLibrary.Array_Find` _progress))
          (`self.GiveResources` "FIBER" (`KismetArrayLibrary.Array_Find` _progress 1))
          (`self.GiveResources` "METAL" (`KismetArrayLibrary.Array_Find` _progress 2)))))))

(event `self.ReceiveBeginPlay`
  (bind _returnvalue (`KismetSystemLibrary.K2_SetTimerDelegate` (`|CreateDelegate` :!event `Set Widget`) 1.0 true))
  (set `self.Handler Player joined` _returnvalue))

(event `Event Add Resources`
  (params (`Resource Type` :type "EResources Enum" :default "WOOD") (Amount :type Integer))
  (`self.GiveResources` `Resource Type` Amount))

(event `CustomEvent`
  (params (NewParam :type "EResources Enum" :default "WOOD") (NewParam2 :type Integer))
  (`self.MC_GiveResource` NewParam NewParam2))

(event `self.Throw_Hitbox.OnComponentBeginOverlap`
  (params (OverlappedComponent :type "PrimitiveComponent Object Reference") (OtherActor :type "Actor Object Reference") (OtherComp :type "PrimitiveComponent Object Reference") (OtherBodyIndex :type Integer) (bFromSweep :type Boolean) (SweepResult :type "HitResult Structure (by ref)"))
  (`/Engine/EditorBlueprintResources/ActorMacros.Switch Has Authority`
    (:`Authority`
      (set `self.CanGiveResource` true)
      (bind _asbp_base_resource_chunk (cast `/Game/Racketeers/Blueprints/GatherableItems/BP_BaseResourceChunk` OtherActor))
      (bind _asbp_player (cast `/Game/Racketeers/Core/BP_Player` (`BaseResourceChunk.LastOwner` _asbp_base_resource_chunk)))
      (bind _asbp_player_state (cast `/Game/Racketeers/Characters/Blueprints/BP_PlayerState` (`Pawn.PlayerState` _asbp_player)))
      (set `self.LastPlayerState` _asbp_player_state)
      (bind _returnvalue (`|GetDataTableRow` "/Game/Racketeers/Blueprints/CraftingSystem/DT_CraftableItem.DT_CraftableItem" (`|GetArrayItem` (`self.ListOfUpgrades`)))
        (:`then`
          (for _array_element (break `/Game/Racketeers/Blueprints/CraftingSystem/FCraftableItem` _returnvalue)
            (bind _type (`BaseResourceChunk.type` _asbp_base_resource_chunk))
            (if (and (`|EnumEquality` _type (break `/Game/Racketeers/Blueprints/CraftingSystem/FCraftableResource` _array_element)) (>= (`BlueprintMapLibrary.Map_Find` (`self.NumberOfResources`) (break `/Game/Racketeers/Blueprints/CraftingSystem/FCraftableResource` _array_element)) (`.Amount_5_06530D9145183E861E5874A17EFA2E48` (break `/Game/Racketeers/Blueprints/CraftingSystem/FCraftableResource` _array_element))))
              (set `self.CanGiveResource` false)))
          (if (`self.CanGiveResource`)
            (`self.GiveResources` _type 1)
            (`self.CustomEvent` _type 1)
            (`GameplayStatics.PlaySoundAtLocation` "/Game/Racketeers/Audio/SFX/Environment/SFX_MaterialDeposited.SFX_MaterialDeposited" (`self.K2_GetActorLocation`) (struct) 1.0 1.0 0.0 null null null null)
            (`PrimitiveComponent.SetCollisionEnabled` (`BaseResourceChunk.ResourceMesh` _asbp_base_resource_chunk) "NoCollision")
            (`self.AddCraftingProgress`)
            (`KismetSystemLibrary.Delay` 0.2)
            (`/Engine/EditorBlueprintResources/StandardMacros.IsValid` OtherActor
              (:`Is Valid`
                (`self.K2_DestroyActor` OtherActor)
                (bind _cancraft (`self.CheckIfCanCraft`))
                (if _cancraft
                  (`self.CraftItem`)
                  (`NiagaraFunctionLibrary.SpawnSystemAtLocation` "/Game/Racketeers/Art/Niagara/Crafting/FXS_Workbench.FXS_Workbench" (+ (`self.K2_GetActorLocation`) (0.0 0.0 100.0))))))
            (else
              (`self.Server_ThrowItem` _type _asbp_player)
              (`/Engine/EditorBlueprintResources/StandardMacros.IsValid` _asbp_base_resource_chunk
                (:`Is Valid`
                  (`self.K2_DestroyActor` _asbp_base_resource_chunk))))))))))

(event `MC_GiveResource`
  (params (ResourceType :type "EResources Enum" :default "WOOD") (Amount :type Integer))
  (`/Engine/EditorBlueprintResources/ActorMacros.Switch Has Authority`
    (:`Remote`
      (`self.GiveResources` ResourceType Amount)
      (`GameplayStatics.PlaySoundAtLocation` "/Game/Racketeers/Audio/SFX/Environment/SFX_MaterialDeposited.SFX_MaterialDeposited" (`self.K2_GetActorLocation`) (struct) 1.0 1.0 0.0 null null null null)
      (bind _cancraft (`self.CheckIfCanCraft`))
      (if _cancraft
        (`self.CraftItem`)))))

(event `Server_CraftItem`
  (`self.MC_CraftItem`))

(event `MC_CraftItem`
  (`self.CraftItem`)
  (`NiagaraFunctionLibrary.SpawnSystemAtLocation` "/Game/Racketeers/Art/Niagara/Crafting/FXS_Workbench.FXS_Workbench" (+ (`self.K2_GetActorLocation`) (0.0 0.0 100.0))))

(event `Server_ThrowItem`
  (params (ResourceType :type "EResources Enum" :default "WOOD") (Player :type "/Game/Racketeers/Core/BP_Player Object Reference"))
  (`self.ThrowBackItem` ResourceType Player))

(event `Interact`
  (params (Instigator :type "Actor Object Reference"))
  (bind _asbp_player (cast `/Game/Racketeers/Core/BP_Player` Instigator))
  (bind _asbp_player_state (cast `/Game/Racketeers/Characters/Blueprints/BP_PlayerState` (`Pawn.PlayerState` _asbp_player)))
  (set `self.LastPlayerState` _asbp_player_state)
  (bind (_holdingresourceinfo_resource _holdingresourceinfo_amount) (break `/Game/Racketeers/Blueprints/CraftingSystem/FCraftableResource` (`/Game/Racketeers/Core/BP_Player.HoldingResourceInfo` _asbp_player)))
  (if (`|EnumInequality` _holdingresourceinfo_resource "NONE")
    (bind _returnvalue (`|GetDataTableRow` "/Game/Racketeers/Blueprints/CraftingSystem/DT_CraftableItem.DT_CraftableItem" (`|GetArrayItem` (`self.ListOfUpgrades`)))
      (:`then`
        (for _array_element (break `/Game/Racketeers/Blueprints/CraftingSystem/FCraftableItem` _returnvalue)
          (if (and (`|EnumEquality` _holdingresourceinfo_resource (break `/Game/Racketeers/Blueprints/CraftingSystem/FCraftableResource` _array_element)) (>= (`BlueprintMapLibrary.Map_Find` (`self.NumberOfResources`) (break `/Game/Racketeers/Blueprints/CraftingSystem/FCraftableResource` _array_element)) (`.Amount_5_06530D9145183E861E5874A17EFA2E48` (break `/Game/Racketeers/Blueprints/CraftingSystem/FCraftableResource` _array_element))))
            (set `self.CanGiveResource` false)))
        (if (`self.CanGiveResource`)
          (`self.GiveResources` _holdingresourceinfo_resource _holdingresourceinfo_amount)
          (`GameplayStatics.PlaySoundAtLocation` "/Game/Racketeers/Audio/SFX/Environment/SFX_MaterialDeposited.SFX_MaterialDeposited" (`self.K2_GetActorLocation`) (struct) 1.0 1.0 0.0 null null null null)
          (set `/Game/Racketeers/Core/BP_Player.HoldingResourceInfo` (make `/Game/Racketeers/Blueprints/CraftingSystem/FCraftableResource` "NONE") _asbp_player)
          (`StaticMeshComponent.SetStaticMesh` (`/Game/Racketeers/Core/BP_Player.HoldingObject` _asbp_player) null)
          (set `/Game/Racketeers/Core/BP_Player.CanChargeThrow` false _asbp_player)
          (`ActorComponent.Deactivate` (`/Game/Racketeers/Core/BP_Player.Sparkle_Effect` _asbp_player))
          (set `/Game/Racketeers/Core/BP_Player.IsHoldingResource` false _asbp_player)
          (bind _cancraft (`self.CheckIfCanCraft`))
          (if _cancraft
            (`self.CraftItem`)
            (`NiagaraFunctionLibrary.SpawnSystemAtLocation` "/Game/Racketeers/Art/Niagara/Crafting/FXS_Workbench.FXS_Workbench" (+ (`self.K2_GetActorLocation`) (0.0 0.0 100.0)))))))))

(fn `AddCraftingProgress`
  (bind _numberofresources (`self.NumberOfResources`))
  (bind _asbp_base_game_state (cast `/Game/Racketeers/Core/Framework/BP_BaseGameState` (`GameplayStatics.GetGameState`)))
  (`RacketeersGameStateBase.AddCraftingProgress` _asbp_base_game_state (`self.Team`) (`self.BenchType`) (`|MakeArray` (`BlueprintMapLibrary.Map_Find` _numberofresources "WOOD") (`BlueprintMapLibrary.Map_Find` _numberofresources "FIBER") (`BlueprintMapLibrary.Map_Find` _numberofresources "METAL"))))

(fn `CheckIfCanCraft`
  (returns (CanCraft :type Boolean))
  (bind _listofupgrades (`self.ListOfUpgrades`))
  (if (`KismetArrayLibrary.Array_IsValidIndex` _listofupgrades)
    (bind _returnvalue (`|GetDataTableRow` "/Game/Racketeers/Blueprints/CraftingSystem/DT_CraftableItem.DT_CraftableItem" (`|GetArrayItem` _listofupgrades))
      (:`then`
        (set `self.IsCraftSuccesful` true)
        (bind (_resources _craftingtable) (break `/Game/Racketeers/Blueprints/CraftingSystem/FCraftableItem` _returnvalue))
        (if (`|EnumEquality` _craftingtable (`self.BenchType`))
          (for _array_element _resources
            (bind (_resource _amount) (break `/Game/Racketeers/Blueprints/CraftingSystem/FCraftableResource` _array_element))
            (bind (_value _returnvalue_2) (`BlueprintMapLibrary.Map_Find` (`self.NumberOfResources`) _resource))
            (if (not (and _returnvalue_2 (>= _value _amount)))
              (set `self.IsCraftSuccesful` false)))
          (return (`self.IsCraftSuccesful`))
          (else
            (return false))))
      (:`RowNotFound`
        (return false)))
    (else
      (return false))))

(fn `CraftItem`
  (bind _returnvalue (`|GetDataTableRow` "/Game/Racketeers/Blueprints/CraftingSystem/DT_CraftableItem.DT_CraftableItem" (`|GetArrayItem` (`self.ListOfUpgrades`)))
    (:`then`
      (bind (_resources _craftingtable _part) (break `/Game/Racketeers/Blueprints/CraftingSystem/FCraftableItem` _returnvalue))
      (for _array_element _resources
        (bind (_resource _amount) (break `/Game/Racketeers/Blueprints/CraftingSystem/FCraftableResource` _array_element))
        (`self.RemoveResource` _resource _amount))
      (bind _asracketeers_game_state_base (cast `RacketeersGameStateBase` (`GameplayStatics.GetGameState`)))
      (`RacketeersGameStateBase.AddPart` _asracketeers_game_state_base (`self.Team`) (`self.BenchType`) (`KismetMathLibrary.Conv_ByteToInt` _part))
      (`/Engine/EditorBlueprintResources/ActorMacros.Switch Has Authority`
        (:`Authority`
          (`RacketeersGameStateBase.AddCraftingProgress` _asracketeers_game_state_base (`self.Team`) (`self.BenchType`) (`|MakeArray` 0 0 0)))
        (:`Remote`
          _))
      (`KismetArrayLibrary.Array_Remove` (`self.ListOfUpgrades`))
      (`self.UpdateWidget`))))

(fn `GetCraftingProgress`
  (params (GameState :type "/Game/Racketeers/Core/Framework/BP_BaseGameState Object Reference"))
  (returns (Progress :type "Array of Integer"))
  (bind _benchtype (`self.BenchType`))
  (bind (_raccooncraftingprogress_hullprogress _raccooncraftingprogress_cannonprogress _raccooncraftingprogress_sailprogress) (break `TeamCraftingProgress` (`RacketeersGameStateBase.RaccoonCraftingProgress` GameState)))
  (bind (_pandacraftingprogress_hullprogress _pandacraftingprogress_cannonprogress _pandacraftingprogress_sailprogress) (break `TeamCraftingProgress` (`RacketeersGameStateBase.PandaCraftingProgress` GameState)))
  (switch `ETeams` (`self.Team`)
    (:`Team_Raccoon`
      (switch `EPartSpacing` _benchtype
        (:`HULL`
          (return _raccooncraftingprogress_hullprogress))
        (:`CANNON`
          (return _raccooncraftingprogress_cannonprogress))
        (:`SAIL`
          (return _raccooncraftingprogress_sailprogress))))
    (:`Team_Panda`
      (switch `EPartSpacing` _benchtype
        (:`HULL`
          (return _pandacraftingprogress_hullprogress))
        (:`CANNON`
          (return _pandacraftingprogress_cannonprogress))
        (:`SAIL`
          (return _pandacraftingprogress_sailprogress))))))

(fn `GetTeamPart`
  (params (GameState :type "/Game/Racketeers/Core/Framework/BP_BaseGameState Object Reference"))
  (returns (Part :type Byte))
  (bind (_raccoonparts_hull _raccoonparts_cannon _raccoonparts_sail) (break `TeamShipParts` (`RacketeersGameStateBase.RaccoonParts` GameState)))
  (bind (_pandasparts_hull _pandasparts_cannon _pandasparts_sail) (break `TeamShipParts` (`RacketeersGameStateBase.PandasParts` GameState)))
  (bind _benchtype (`self.BenchType`))
  (switch `ETeams` (`self.Team`)
    (:`Team_Raccoon`
      (switch `EPartSpacing` _benchtype
        (:`HULL`
          (return _raccoonparts_hull))
        (:`CANNON`
          (return _raccoonparts_cannon))
        (:`SAIL`
          (return _raccoonparts_sail))))
    (:`Team_Panda`
      (switch `EPartSpacing` _benchtype
        (:`HULL`
          (return _pandasparts_hull))
        (:`CANNON`
          (return _pandasparts_cannon))
        (:`SAIL`
          (return _pandasparts_sail))))))

(fn `GiveResources`
  (params (`Resource Type` :type "EResources Enum" :default "WOOD") (Amount :type Integer))
  (locals (ResourceType :type "EResources Enum" :default "WOOD"))
  (bind _numberofresources (`self.NumberOfResources`))
  (set `local.ResourceType` `Resource Type`)
  (if (`BlueprintMapLibrary.Map_Contains` _numberofresources (`local.ResourceType`))
    (`BlueprintMapLibrary.Map_Add` (`self.NumberOfResources`) (`local.ResourceType`) (+ (`BlueprintMapLibrary.Map_Find` _numberofresources (`local.ResourceType`)) Amount))
    (else
      (`BlueprintMapLibrary.Map_Add` (`self.NumberOfResources`) (`local.ResourceType`) Amount)))
  (bind _returnvalue (`|GetDataTableRow` "/Game/Racketeers/Blueprints/CraftingSystem/DT_CraftableItem.DT_CraftableItem" (`|GetArrayItem` (`self.ListOfUpgrades`)))
    (:`then`
      (for _array_element (`.Resources_3_CFA65A04420AD933476066A55C39CB0A` (break `/Game/Racketeers/Blueprints/CraftingSystem/FCraftableItem` _returnvalue))
        (bind (_resource _amount) (break `/Game/Racketeers/Blueprints/CraftingSystem/FCraftableResource` _array_element))
        (if (`|EnumEquality` _resource (`local.ResourceType`))
          (bind _aswbp_work_bench_part_world_cannon (cast `/Game/Racketeers/Blueprints/Widgets/WorkBench/WBP_WorkBenchPart_World_Cannon` (`WidgetComponent.GetUserWidgetObject` (`self.Widget`))))
          (`/Game/Racketeers/Blueprints/Widgets/WorkBench/WBP_WorkBenchPart_World_Cannon.LowerRequierment` _aswbp_work_bench_part_world_cannon (`local.ResourceType`) (- _amount (`BlueprintMapLibrary.Map_Find` (`self.NumberOfResources`) (`local.ResourceType`)))))))))

(fn `RemoveResource`
  (params (ResourceType :type "EResources Enum" :default "WOOD") (Amount :type Integer))
  (bind (_value _returnvalue) (`BlueprintMapLibrary.Map_Find` (`self.NumberOfResources`) ResourceType))
  (bind _returnvalue_2 (- _value Amount))
  (if _returnvalue
    (if (<= _returnvalue_2 0)
      (`BlueprintMapLibrary.Map_Add` (`self.NumberOfResources`) ResourceType)
      (else
        (`BlueprintMapLibrary.Map_Add` (`self.NumberOfResources`) ResourceType _returnvalue_2)))))

(fn `ThrowBackItem`
  (params (ResourceType :type "EResources Enum" :default "WOOD") (Player :type "/Game/Racketeers/Core/BP_Player Object Reference"))
  (locals (`Spawning Class` :type "/Game/Racketeers/Blueprints/GatherableItems/BP_BaseResourceChunk Class Reference"))
  (bind (_returnvalue_location _returnvalue_rotation) (`KismetMathLibrary.BreakTransform` (`SceneComponent.K2_GetComponentToWorld` (`self.ThrowBack_Location`))))
  (`|ExecutionSequence`
    (:`then_0`
      (switch `EResources` ResourceType
        (:`WOOD`
          (set `local.Spawning Class` "/Game/Racketeers/Blueprints/GatherableItems/BP_BaseResourceChunkWood.BP_BaseResourceChunkWood_C"))
        (:`FIBER`
          (set `local.Spawning Class` "/Game/Racketeers/Blueprints/GatherableItems/BP_BaseResourceChunkFiber.BP_BaseResourceChunkFiber_C"))
        (:`METAL`
          (set `local.Spawning Class` "/Game/Racketeers/Blueprints/GatherableItems/BP_BaseResourceChunkMetal.BP_BaseResourceChunkMetal_C"))))
    (:`then_1`
      (bind _returnvalue (`|SpawnActorFromClass` (`local.Spawning Class`) (`KismetMathLibrary.MakeTransform` _returnvalue_location _returnvalue_rotation) "Undefined" "MultiplyWithRoot" null (1.0 0.0 0.0) 1000.0 null))
      (set `/Game/Racketeers/Blueprints/GatherableItems/BP_BaseResourceChunk.MaxSpeed` 1000.0 _returnvalue)
      (set `BaseResourceChunk.isBeingHeld` false _returnvalue)
      (set `BaseResourceChunk.LastOwner` Player _returnvalue))))

(fn `UpdateWidget`
  (bind _aswbp_work_bench_part_world_cannon (cast `/Game/Racketeers/Blueprints/Widgets/WorkBench/WBP_WorkBenchPart_World_Cannon` (`WidgetComponent.GetUserWidgetObject` (`self.Widget`))))
  (`/Game/Racketeers/Blueprints/Widgets/WorkBench/WBP_WorkBenchPart_World_Cannon.UpdateWidget` _aswbp_work_bench_part_world_cannon "NewEnumerator0" (`|GetArrayItem` (`self.ListOfUpgrades`))))

(fn `UserConstructionScript`)
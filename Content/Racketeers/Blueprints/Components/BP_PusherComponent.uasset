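; Pusher component that lets its owner shove a player just in front of it, stunning and launching them.
; Push sphere-traces ahead, then plays push and hit sounds, calls PushStun, server-throws any held resource upward, launches the victim and turns them opposite the owner's facing.
; A shove effect spawns near the victim on all clients, while a DoOnce reset after PushCooldown limits repeat hits.
; The multicast item-throw path is marked old.
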(event `Push Sound`
  (`GameplayStatics.PlaySoundAtLocation` "/Game/Racketeers/Audio/SFX/Player/SFX_PlayerPushAbstract.SFX_PlayerPushAbstract" (`Actor.K2_GetActorLocation` (`self.GetOwner`)) (struct) 1.0 1.0 0.0 null null null null))

(event `HitSound`
  (params (Location :type "Vector Structure"))
  (`GameplayStatics.PlaySoundAtLocation` "/Game/Racketeers/Audio/SFX/Player/SFX_PlayerHit.SFX_PlayerHit" Location (struct) 1.0 1.0 0.0 null null null null))

(event `Push`
  (bind _returnvalue (`self.GetOwner`))
  (bind _returnvalue_2 (`self.GetOwner`))
  (bind _returnvalue_3 (`Actor.K2_GetActorLocation` _returnvalue))
  (bind (_returnvalue_x _returnvalue_y) (`KismetMathLibrary.BreakVector` (* (`Actor.GetActorForwardVector` _returnvalue) 1500.0)))
  (bind _returnvalue_4 (+ (`Actor.K2_GetActorLocation` _returnvalue_2) (* (`Actor.GetActorForwardVector` _returnvalue_2) 100.0)))
  (bind (_outhit _returnvalue_5) (`KismetSystemLibrary.SphereTraceSingleForObjects` :`Start` _returnvalue_4 :`End` _returnvalue_4 :`Radius` 64.0 :`ObjectTypes` (`|MakeArray` "ObjectTypeQuery8" "ObjectTypeQuery7" :!type "EObjectTypeQuery Enum") :`DrawTime` 2.0))
  (if _returnvalue_5
    (`/Engine/EditorBlueprintResources/StandardMacros.DoOnce` false :!label _label
      (:`Completed`
        (`self.Push Sound`)
        (bind (_bblockinghit _binitialoverlap _time _distance _location _impactpoint _normal _impactnormal _physmat _hitactor) (`GameplayStatics.BreakHitResult` _outhit))
        (`self.HitSound` (`Actor.K2_GetActorLocation` _hitactor))
        (set `self.IsPushing` true)
        (bind _asbp_player (cast `/Game/Racketeers/Core/BP_Player` _hitactor))
        (`/Game/Racketeers/Core/BP_Player.Push_Stun` _asbp_player)
        (`KismetSystemLibrary.Delay` 0.1)
        (bind (_holdingresourceinfo_resource _holdingresourceinfo_amount) (break `/Game/Racketeers/Blueprints/CraftingSystem/FCraftableResource` (`/Game/Racketeers/Core/BP_Player.HoldingResourceInfo` _asbp_player)))
        (if (> _holdingresourceinfo_amount 0)
          (`/Game/Racketeers/Core/BP_Player.Server_Throw` _asbp_player _asbp_player 0.0 true))
        (`Character.LaunchCharacter` _asbp_player (`KismetMathLibrary.MakeVector` _returnvalue_x _returnvalue_y 250.0) true true)
        (`Actor.K2_SetActorRotation` _asbp_player (`KismetMathLibrary.MakeRotator` (.roll (`Actor.K2_GetActorRotation` _returnvalue)) (.pitch (`Actor.K2_GetActorRotation` _returnvalue)) (+ (.yaw (`Actor.K2_GetActorRotation` _returnvalue)) 180.0)) false)
        (bind _returnvalue_6 (`Actor.K2_GetActorLocation` _asbp_player))
        (`self.MC_Spawn_Effect` (- _returnvalue_3 (* (`KismetMathLibrary.Normal` (- _returnvalue_3 _returnvalue_6)) (- (`KismetMathLibrary.Vector_Distance` _returnvalue_3 _returnvalue_6) 50.0))))
        (`KismetSystemLibrary.Delay` 0.3)
        (set `self.IsPushing` false)
        (`KismetSystemLibrary.Delay` (- (`self.PushCooldown`) 0.3))
        (goto _label :!via `Reset`)))))

(event `MC_Spawn_Effect`
  (params (LaunchedCharacter :type "Vector Structure"))
  ;[1 1 1] Spawn effect at location for all clients
  (`self.Spawn_Effect` LaunchedCharacter))

(event `Spawn_Effect`
  (params (LaunchedCharacter :type "Vector Structure"))
  ;[1 1 1] Spawn effect at location for all clients
  (`NiagaraFunctionLibrary.SpawnSystemAtLocation` "/Game/Racketeers/Art/Niagara/Player/FXS_Shove.FXS_Shove" LaunchedCharacter))

(event `MC_ThrowItem`
  (params (Player :type "/Game/Racketeers/Core/BP_Player Object Reference"))
  ;[1 1 1] Throws the item on push on all clients (OLD)
  (`self.ThrowItem_Event` Player))

(event `ThrowItem_Event`
  (params (Player :type "/Game/Racketeers/Core/BP_Player Object Reference"))
  ;[1 1 1] Throws the item on push on all clients (OLD)
  (`/Game/Racketeers/Core/BP_Player.ThrowResource` Player true null 0.0))
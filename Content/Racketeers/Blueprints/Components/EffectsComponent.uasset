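; Actor component in Racketeers that triggers particle effects and a stun sound for its owner.
; Server-named events forward to multicast-named events, which restart the passed Stress and Running particle components or spawn a given system at a position.
; StunAudio stands apart from that relay and plays the player-stunned sound directly at the owner's location.
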(event `ServerRunningEffects`
  (params (Stress :type "NiagaraComponent Object Reference") (Running :type "NiagaraComponent Object Reference"))
  (`self.MultiCastRunningEffects` Stress Running))

(event `MultiCastRunningEffects`
  (params (Stress :type "NiagaraComponent Object Reference") (Running :type "NiagaraComponent Object Reference"))
  (`NiagaraComponent.ReinitializeSystem` Stress)
  (`NiagaraComponent.ReinitializeSystem` Running))

(event `ServerOneEffectCall`
  (params (Stress :type "NiagaraComponent Object Reference"))
  (`self.MultiOneEffectCall` Stress))

(event `MultiOneEffectCall`
  (params (Stress :type "NiagaraComponent Object Reference"))
  (`NiagaraComponent.ReinitializeSystem` Stress))

(event `ServerSpawnAtEffectAtPosition`
  (params (Effect :type "NiagaraSystem Object Reference") (Position :type "Vector Structure"))
  (`self.MultiSpawnAtEffectAtPosition` Effect Position))

(event `MultiSpawnAtEffectAtPosition`
  (params (Effect :type "NiagaraSystem Object Reference") (Postion :type "Vector Structure"))
  (`NiagaraFunctionLibrary.SpawnSystemAtLocation` Effect Postion))

(event `StunAudio`
  (`GameplayStatics.PlaySoundAtLocation` "/Game/Racketeers/Audio/SFX/Player/SFX_PlayerStunned.SFX_PlayerStunned" (`Actor.K2_GetActorLocation` (`self.GetOwner`)) (struct) 1.0 1.0 0.0 null null null null))
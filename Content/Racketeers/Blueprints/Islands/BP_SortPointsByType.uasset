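; Custom PCG Blueprint node that randomly splits input points into tree, bush and rock spawn points for island resources.
; GenerateRatio divides each ResourceTable value by the table's entry count, not the sum of its values.
; ExecuteWithContext multiplies each ratio by ResourceAmount, rounds up, and draws that many random points without replacement.
; Wood, fiber and metal picks become separate point data on the TreePoints, BushPoints and RockPoints pins.
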(fn ExecutewithContext
  (params (InContext :type PCG%20Context%20Structure%20%28by%20ref%29) (Input :type PCG%20Data%20Collection%20Structure%20%28by%20ref%29))
  ;[1 1 1] Get Points
  (bind _returnvalue (Data|GetTypedInputsbyPinLabel Input "In" "/Script/PCG.PCGPointData"))
  (for _array_element _returnvalue
    (bind _output_get (LocalVariables|SetInPointData _array_element))
    (LocalVariables|SetInPoints (SpatialData|GetPoints _output_get))
    ;[1 1 1] Generate Ratio table
    (bind _resourceratiotable (CallFunction|GenerateRatio (Variables|Default|GetResourceTable)))
    (bind _output_get_2 (LocalVariables|SetResourceRatio _resourceratiotable))
    (bind _keys (Utilities|Map|Keys _output_get_2))
    ;[1 1 1] Forloop
    (for _array_element_2 _keys
      (bind _output_get_3 (LocalVariables|SetCurrentResource _array_element_2))
      (if (.ReturnValue (Utilities|Map|Find (LocalVariables|GetResourceRatio) _output_get_3))
        ;;[1 1 1] Forloop
        (for _index (range 1 (Math|Float|Ceil (* (Math|Conversions|ToFloat(Integer) (Variables|Default|GetResourceAmount)) (.Value (Utilities|Map|Find (LocalVariables|GetResourceRatio) _output_get_3)))))
          (if (Utilities|Array|IsNotEmpty (LocalVariables|GetInPoints))
            (bind _output_get_4 (LocalVariables|SetCurrentPoint (Utilities|Array|Get(acopy) (LocalVariables|GetInPoints) (Math|Random|RandomIntegerinRange 0 (- (Utilities|Array|Length (LocalVariables|GetInPoints)) 1)))))
            (bind _returnvalue_2 (Utilities|Array|RemoveItem (LocalVariables|GetInPoints) _output_get_4))
            (if _returnvalue_2
              _
              (else
                _))
            (switch Utilities|FlowControl|Switch|SwitchonEResources (LocalVariables|GetCurrentResource)
              (:WOOD
                (Utilities|Array|AddUnique (LocalVariables|GetTreePoints) (LocalVariables|GetCurrentPoint)))
              (:FIBER
                (Utilities|Array|AddUnique (LocalVariables|GetBushPoints) (LocalVariables|GetCurrentPoint)))
              (:METAL
                (Utilities|Array|AddUnique (LocalVariables|GetRockPoints) (LocalVariables|GetCurrentPoint))))))
        (else
          (Development|PrintString "Did not find a type"))))
    ;[1 1 1] Creates OutputData
    (Utilities|FlowControl|Sequence
      (:then_0
        (bind _returnvalue_3 (Game|ConstructObjectfromClass "/Script/PCG.PCGPointData"))
        (bind _output_get_5 (LocalVariables|SetTreePointData _returnvalue_3))
        (SpatialData|InitializefromData _output_get_5 (LocalVariables|GetInPointData) 0 true true)
        (SpatialData|SetPoints (LocalVariables|GetTreePointData) (LocalVariables|GetTreePoints))
        (Class|PCGDataFunctionLibrary|AddtoCollection (LocalVariables|GetOutPutCollection) (LocalVariables|GetTreePointData) "TreePoints" (Utilities|Array|MakeArray "")))
      (:then_1
        (bind _returnvalue_4 (Game|ConstructObjectfromClass "/Script/PCG.PCGPointData"))
        (bind _output_get_6 (LocalVariables|SetRockPointData _returnvalue_4))
        (SpatialData|InitializefromData _output_get_6 (LocalVariables|GetInPointData) 0 true true)
        (SpatialData|SetPoints (LocalVariables|GetRockPointData) (LocalVariables|GetRockPoints))
        (Class|PCGDataFunctionLibrary|AddtoCollection (LocalVariables|GetOutPutCollection) (LocalVariables|GetRockPointData) "RockPoints" (Utilities|Array|MakeArray "")))
      (:then_2
        (bind _returnvalue_5 (Game|ConstructObjectfromClass "/Script/PCG.PCGPointData"))
        (bind _output_get_7 (LocalVariables|SetBushPointData _returnvalue_5))
        (SpatialData|InitializefromData _output_get_7 (LocalVariables|GetInPointData) 0 true true)
        (SpatialData|SetPoints (LocalVariables|GetBushPointData) (LocalVariables|GetBushPoints))
        (Class|PCGDataFunctionLibrary|AddtoCollection (LocalVariables|GetOutPutCollection) (LocalVariables|GetBushPointData) "BushPoints" (Utilities|Array|MakeArray "")))))
  ;[1 1 1] Returns the collection data.
  (return (LocalVariables|GetOutPutCollection)))

(fn GenerateRatio
  (params (InputResourceTable :type Map%20of%20EResources%20Enums%20to%20Integers :default "WOOD"))
  (bind _keys (Utilities|Map|Keys InputResourceTable))
  (for _array_element _keys
    (if (.ReturnValue (Utilities|Map|Find InputResourceTable _array_element))
      (Utilities|Map|Add (LocalVariables|GetRatioTable) _array_element (/ (Math|Conversions|ToFloat(Integer) (.Value (Utilities|Map|Find InputResourceTable _array_element))) (Math|Conversions|ToFloat(Integer) (Utilities|Map|Length InputResourceTable))))))
  (return (LocalVariables|GetRatioTable)))
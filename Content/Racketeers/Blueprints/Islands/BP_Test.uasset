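; Custom PCG node that scatters wood, fiber and metal resource points as trees, bushes and rocks.
; GatherPoints draws random input points up to each ResourceTable count, removing accepted ones and retrying rejects without an attempt limit.
; Candidates must clear placed points by summed ResourceRadius values, although the rock check uses the FIBER radius.
; Results go to TreePoints, BushPoints and RockPoints output pins.
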(fn ExecutewithContext
  (params (InContext :type PCG%20Context%20Structure%20%28by%20ref%29) (Input :type PCG%20Data%20Collection%20Structure%20%28by%20ref%29))
  ;[1 1 1] Get Input points
  (bind _returnvalue (Data|GetTypedInputsbyPinLabel Input "In" "/Script/PCG.PCGPointData"))
  (for _array_element _returnvalue
    (bind _output_get (Variables|Default|SetInPointData _array_element))
    (Variables|Default|SetInPoints (SpatialData|GetPoints _output_get))
    (Utilities|FlowControl|Sequence
      (:then_0
        (CallFunction|GatherPoints (Variables|Default|GetTreePoints) "WOOD"))
      (:then_1
        (CallFunction|GatherPoints (Variables|Default|GetBushPoints) "FIBER"))
      (:then_2
        (CallFunction|GatherPoints (Variables|Default|GetRockPoints) "METAL"))))
  (Utilities|FlowControl|Sequence
    (:then_0
      (bind _returnvalue_2 (Game|ConstructObjectfromClass "/Script/PCG.PCGPointData"))
      (bind _output_get_2 (LocalVariables|SetTreePointData _returnvalue_2))
      (SpatialData|InitializefromData _output_get_2 (Variables|Default|GetInPointData) 0 true true)
      (SpatialData|SetPoints (LocalVariables|GetTreePointData) (Variables|Default|GetTreePoints))
      (Class|PCGDataFunctionLibrary|AddtoCollection (LocalVariables|GetOutputCollection) (LocalVariables|GetTreePointData) "TreePoints" (Utilities|Array|MakeArray "")))
    (:then_1
      (bind _returnvalue_3 (Game|ConstructObjectfromClass "/Script/PCG.PCGPointData"))
      (bind _output_get_3 (LocalVariables|SetBushPointData _returnvalue_3))
      (SpatialData|InitializefromData _output_get_3 (Variables|Default|GetInPointData) 0 true true)
      (SpatialData|SetPoints (LocalVariables|GetBushPointData) (Variables|Default|GetBushPoints))
      (Class|PCGDataFunctionLibrary|AddtoCollection (LocalVariables|GetOutputCollection) (LocalVariables|GetBushPointData) "BushPoints" (Utilities|Array|MakeArray "")))
    (:then_2
      (bind _returnvalue_4 (Game|ConstructObjectfromClass "/Script/PCG.PCGPointData"))
      (bind _output_get_4 (LocalVariables|SetRockPointData _returnvalue_4))
      (SpatialData|InitializefromData _output_get_4 (Variables|Default|GetInPointData) 0 true true)
      (SpatialData|SetPoints (LocalVariables|GetRockPointData) (Variables|Default|GetRockPoints))
      (Class|PCGDataFunctionLibrary|AddtoCollection (LocalVariables|GetOutputCollection) (LocalVariables|GetRockPointData) "RockPoints" (Utilities|Array|MakeArray "")))
    (:then_3
      (return (LocalVariables|GetOutputCollection)))))

(fn CheckDistance
  (params (Point :type PCG%20Point%20Structure) (PointArray :type Array%20of%20PCG%20Point%20Structures) (ResourceToCheck :type EResources%20Enum :default "WOOD") (ArrayType :type EResources%20Enum :default "WOOD"))
  (bind _resourceradius (Variables|Default|GetResourceRadius))
  (if (Utilities|Array|IsNotEmpty PointArray)
    (for _array_element PointArray
      (if (not (> (Math|Vector|Distance(Vector) (.location (.Transform (Utilities|Struct|BreakPCGPoint Point))) (.location (.Transform (Utilities|Struct|BreakPCGPoint _array_element)))) (+ (.Value (Utilities|Map|Find _resourceradius ResourceToCheck)) (.Value (Utilities|Map|Find _resourceradius ArrayType)))))
        (return false)))
    (return true)
    (else
      (return true))))

(fn GetValidRandomPoint
  (params (PointArray :type Array%20of%20PCG%20Point%20Structures))
  (return (Utilities|Array|Get(acopy) (Variables|Default|GetInPoints) (Math|Random|RandomIntegerinRange 0 (- (Utilities|Array|Length PointArray) 1)))))

(fn ValidatePoint
  (params (Point :type PCG%20Point%20Structure) (Type :type EResources%20Enum :default "WOOD"))
  (Utilities|FlowControl|Sequence
    (:then_0
      (bind _distancecheck (CallFunction|CheckDistance Point (Variables|Default|GetTreePoints) Type "WOOD"))
      (bind _output_get (LocalVariables|SetTreeDistanceCheck _distancecheck))
      (if (not _output_get)
        (return false)))
    (:then_1
      (bind _distancecheck_2 (CallFunction|CheckDistance Point (Variables|Default|GetBushPoints) Type "FIBER"))
      (bind _output_get_2 (LocalVariables|SetBushDIstanceCheck _distancecheck_2))
      (if (not _output_get_2)
        (return false)))
    (:then_2
      (bind _distancecheck_3 (CallFunction|CheckDistance Point (Variables|Default|GetRockPoints) Type "FIBER"))
      (bind _output_get_3 (LocalVariables|SetRockDistanceCheck _distancecheck_3))
      (if (not _output_get_3)
        (return false)))
    (:then_3
      (if (Math|Boolean|ANDBoolean (LocalVariables|GetTreeDistanceCheck) (LocalVariables|GetBushDIstanceCheck) (LocalVariables|GetRockDistanceCheck))
        (return true)
        (else
          (return false))))))

(fn GatherPoints
  (params (PointArray :type Array%20of%20PCG%20Point%20Structures) (ArrayType :type EResources%20Enum :default "WOOD"))
  (bind _resourcetable (Variables|Default|GetResourceTable))
  (bind (_value _returnvalue) (Utilities|Map|Find _resourcetable ArrayType))
  (if _returnvalue
    (for _index (range 1 _value)
      (LocalVariables|Setb true)
      (while (LocalVariables|Getb)
        (bind _point (CallFunction|GetValidRandomPoint (Variables|Default|GetInPoints)))
        (bind _output_get (LocalVariables|SetCurrentPointLocal _point))
        (bind _isvalid (CallFunction|ValidatePoint _output_get ArrayType))
        (if _isvalid
          (bind _updated (CallFunction|UpdateArray PointArray (LocalVariables|GetCurrentPointLocal)))
          (LocalVariables|Setb (not _updated))
          (else
            (Development|PrintString "Too close"))))))
  (return))

(fn UpdateArray
  (params (ArrayToUpdate :type Array%20of%20PCG%20Point%20Structures) (CurrentPoint :type PCG%20Point%20Structure))
  (Utilities|Array|Add ArrayToUpdate CurrentPoint)
  (bind _returnvalue (Utilities|Array|RemoveItem (Variables|Default|GetInPoints) CurrentPoint))
  (return _returnvalue))
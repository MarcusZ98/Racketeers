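; Custom PCG Blueprint element that scatters tree, bush and rock resource actors across an island's PCG points.
; PointLoopBody collects unique point transforms, then on the server GenerateResources splits the island tier's total by base ratios plus random shares.
; SpawnResource places each type at random collected transforms, removing each from the pool and recording it per type.
; Both server and client return the point loop's data to the graph.
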(fn ExecutewithContext
  (params (InContext :type PCG%20Context%20Structure%20%28by%20ref%29) (Input :type PCG%20Data%20Collection%20Structure%20%28by%20ref%29))
  ;[1 1 1] Gets all points
  (bind _returnvalue (Class|PCGDataFunctionLibrary|GetInputs Input))
  (bind _aspcgspatial_data (Utilities|Casting|CastToPCGSpatialData (.Data (Utilities|Struct|BreakPCGTaggedData (Utilities|Array|Get(acopy) _returnvalue))))
    (:then
      ;[1 1 1] Calls PointLoopBody Function
      (bind _outdata (PCG|FlowControl|PointLoop InContext (SpatialData|ToPointDatawithContext _aspcgspatial_data InContext) 0))
      ;[1 1 1] Check if the function is called by the server
      (if (Networking|IsServer)
        ;[1 1 1] Generate resources
        (bind (_trees _bushes _rocks) (CallFunction|GenerateResources (Variables|Default|GetIslandEnumTier)))
        (Utilities|FlowControl|Sequence
          (:then_0
            (CallFunction|SpawnResource _trees "WOOD"))
          (:then_1
            (CallFunction|SpawnResource _bushes "FIBER"))
          (:then_2
            (CallFunction|SpawnResource _rocks "METAL"))
          (:then_3
            (return (Utilities|Struct|MakePCGDataCollection (Utilities|Array|MakeArray (Utilities|Struct|MakePCGTaggedData _outdata 0 "None"))))))
        (else
          (return (Utilities|Struct|MakePCGDataCollection (Utilities|Array|MakeArray (Utilities|Struct|MakePCGTaggedData _outdata 0 "None")))))))
    (:CastFailed
      (return ""))))

(fn PointLoopBody
  (params (InContext :type PCG%20Context%20Structure%20%28by%20ref%29) (InData :type PCG%20Point%20Data%20Object%20Reference) (InPoint :type PCG%20Point%20Structure%20%28by%20ref%29) (OutMetadata :type PCG%20Metadata%20Object%20Reference) (Iteration :type Integer64))
  ;[1 1 1] Runs for every point
  (Utilities|Array|AddUnique (Variables|Default|GetPointLocations) (.transform InPoint))
  (return (Utilities|Struct|MakePCGPoint (.transform InPoint) (.density InPoint) (.boundsmin InPoint) (.boundsmax InPoint) (.color InPoint) (.steepness InPoint) (.seed InPoint)) false))

(fn GenerateResources
  (params (IslandTier :type ETier%20Enum :default "NewEnumerator3"))
  (bind _tiervalue (LocalVariables|GetTierValue))
  (bind _value (Utilities|Map|Find _tiervalue IslandTier))
  (if (Utilities|Enum|Equal(Enum) IslandTier "NewEnumerator3")
    (return 0 0 0)
    (else
      (bind _output_get (LocalVariables|SetRemainingRatio (- (LocalVariables|GetRemainingRatio) (+ (LocalVariables|GetTreeRatio) (LocalVariables|GetBushRatio) (LocalVariables|GetRockRatio)))))
      (LocalVariables|SetTreeRatio (+ (LocalVariables|GetTreeRatio) (Math|Random|RandomFloatinRange 0.0 _output_get)))
      (bind _output_get_2 (LocalVariables|SetRemainingRatio (- (LocalVariables|GetRemainingRatio) (Math|Random|RandomFloatinRange 0.0 _output_get))))
      (LocalVariables|SetBushRatio (+ (LocalVariables|GetBushRatio) (Math|Random|RandomFloatinRange 0.0 _output_get_2)))
      (bind _output_get_3 (LocalVariables|SetRemainingRatio (- (LocalVariables|GetRemainingRatio) (Math|Random|RandomFloatinRange 0.0 _output_get_2))))
      (LocalVariables|SetRockRatio (+ (LocalVariables|GetRockRatio) _output_get_3))
      (bind _output_get_4 (LocalVariables|SetRockAmount (Math|Float|Round (* _value (LocalVariables|GetRockRatio)))))
      (bind _output_get_5 (LocalVariables|SetBushAmount (Math|Float|Round (* _value (LocalVariables|GetBushRatio)))))
      (bind _output_get_6 (LocalVariables|SetTreeAmount (Math|Float|Round (* _value (LocalVariables|GetTreeRatio)))))
      (return _output_get_6 _output_get_5 _output_get_4))))

(fn SpawnResource
  (params (AmountToSpawn :type Integer) (Resource :type EResources%20Enum :default "WOOD"))
  ;[1 1 1] Spawn specific amount of resource type
  (for _index (range 1 AmountToSpawn)
    (if (Utilities|Array|IsNotEmpty (Variables|Default|GetPointLocations))
      (bind _availabletransform (CallFunction|GetRandomAvailableIndex))
      (bind _output_get (LocalVariables|SetCurrentTransform _availabletransform))
      (Utilities|Array|RemoveItem (Variables|Default|GetPointLocations) _output_get)
      (switch Utilities|FlowControl|Switch|SwitchonEResources Resource
        (:WOOD
          (Game|SpawnActorfromClass "/Game/Racketeers/Blueprints/GatherableItems/GatherableResource/BP_TreeParent.BP_TreeParent_C" (LocalVariables|GetCurrentTransform) "AlwaysSpawn" "MultiplyWithRoot" 0 0)
          (Utilities|Array|AddUnique (Variables|Default|GetTreeTransforms) (LocalVariables|GetCurrentTransform)))
        (:FIBER
          (Game|SpawnActorfromClass "/Game/Racketeers/Blueprints/GatherableItems/GatherableResource/BP_BushParent.BP_BushParent_C" (LocalVariables|GetCurrentTransform) "AlwaysSpawn" "MultiplyWithRoot" 0 0)
          (Utilities|Array|AddUnique (Variables|Default|GetBushTransforms) (LocalVariables|GetCurrentTransform)))
        (:METAL
          (Game|SpawnActorfromClass "/Game/Racketeers/Blueprints/GatherableItems/GatherableResource/BP_RockParent.BP_RockParent_C" (LocalVariables|GetCurrentTransform) "AlwaysSpawn" "MultiplyWithRoot" 0 0)
          (Utilities|Array|AddUnique (Variables|Default|GetRockTransforms) (LocalVariables|GetCurrentTransform)))))))

(fn GetRandomAvailableIndex
  ;[1 1 1] Returns a avaible TransformPoint
  (return (Utilities|Array|Get(acopy) (Variables|Default|GetPointLocations) (Math|Random|RandomIntegerinRange 0 (- (Utilities|Array|Length (Variables|Default|GetPointLocations)) 1)))))
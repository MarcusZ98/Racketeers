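; Custom PCG node that spawns island resource actors at the incoming points, chosen by its resource Type.
; On the server only, it reads point data from the In pin and spawns a random tree (wood), bush (fiber) or rock (metal) class at each point's transform.
; Spawns adjust for collision but always succeed.
; OutPoints receives only the last point data processed, added after the loop.
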(fn ExecutewithContext
  (params (InContext :type PCG%20Context%20Structure%20%28by%20ref%29) (Input :type PCG%20Data%20Collection%20Structure%20%28by%20ref%29))
  (bind _returnvalue (Data|GetTypedInputsbyPinLabel Input "In" "/Script/PCG.PCGPointData"))
  (if (Networking|IsServer)
    (for _array_element _returnvalue
      (bind _output_get (LocalVariables|SetInPointData _array_element))
      (bind _output_get_2 (LocalVariables|SetInPoints (SpatialData|GetPoints _output_get)))
      (for _array_element_2 _output_get_2
        (LocalVariables|SetCurrentPoint _array_element_2)
        (switch Utilities|FlowControl|Switch|SwitchonEResources (Variables|Default|GetType)
          (:WOOD
            (bind _class (CallFunction|GetRandomClass (LocalVariables|GetTreeActorArray)))
            (Game|SpawnActorfromClass _class (.Transform (Utilities|Struct|BreakPCGPoint (LocalVariables|GetCurrentPoint))) "AdjustIfPossibleButAlwaysSpawn" "MultiplyWithRoot" 0 0))
          (:FIBER
            (bind _class_2 (CallFunction|GetRandomClass (LocalVariables|GetBushActorArray)))
            (Game|SpawnActorfromClass _class_2 (.Transform (Utilities|Struct|BreakPCGPoint (LocalVariables|GetCurrentPoint))) "AdjustIfPossibleButAlwaysSpawn" "MultiplyWithRoot" 0 0))
          (:METAL
            (bind _class_3 (CallFunction|GetRandomClass (LocalVariables|GetRockActorArray)))
            (Game|SpawnActorfromClass _class_3 (.Transform (Utilities|Struct|BreakPCGPoint (LocalVariables|GetCurrentPoint))) "AdjustIfPossibleButAlwaysSpawn" "MultiplyWithRoot" 0 0))
          (:NONE
            (Development|PrintString "No type Selected"))))))
  (Class|PCGDataFunctionLibrary|AddtoCollection (LocalVariables|GetOutputCollection) (LocalVariables|GetInPointData) "OutPoints" (Utilities|Array|MakeArray ""))
  (return (LocalVariables|GetOutputCollection)))

(fn GetRandomClass
  (params (Array :type Array%20of%20Actor%20Class%20References))
  (return (Utilities|Array|Get(acopy) Array (Math|Random|RandomIntegerinRange 0 (- (Utilities|Array|Length Array) 1)))))
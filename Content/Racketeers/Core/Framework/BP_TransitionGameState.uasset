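; Game state for Racketeers phase transitions that shows the stats screen matching the incoming phase.
; On BeginPlay it starts a looping timer, presumably bound to PlayerValid, which polls until the first player controller has a valid PlayerState.
; It then clears the timer and switches on IncomingPhase to create that phase's stats widget for the player and add it to their screen.
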(event `self.ReceiveBeginPlay`
  (bind _returnvalue (`KismetSystemLibrary.K2_SetTimerDelegate` (`|CreateDelegate` :!event `PlayerValid`) 1.0 true true))
  (set `self.CacheHandle` _returnvalue))

(event `PlayerValid`
  (if (`KismetSystemLibrary.IsValid` (`Controller.PlayerState` (`GameplayStatics.GetPlayerController` 0)))
    (`KismetSystemLibrary.K2_ClearAndInvalidateTimerHandle` (`self.CacheHandle`))
    (`self.AddWidgetToScreenWhenPLayerValid`)))

(event `AddWidgetToScreenWhenPLayerValid`
  (`KismetSystemLibrary.PrintString` "Playter Is Valid")
  (switch `EPhaseState` (`self.IncomingPhase`)
    (:`Phase_1`
      (bind _returnvalue (`|CreateWidget` "/Game/Racketeers/Blueprints/Widgets/PhaseWidgets/WBP_Phase1StatsScreen.WBP_Phase1StatsScreen_C" (`GameplayStatics.GetPlayerController` 0)))
      (`UserWidget.AddToPlayerScreen` _returnvalue 0))
    (:`Phase_2`
      (bind _returnvalue_2 (`|CreateWidget` "/Game/Racketeers/Blueprints/Widgets/PhaseWidgets/WBP_Phase2StatsScreen.WBP_Phase2StatsScreen_C" (`GameplayStatics.GetPlayerController` 0)))
      (`UserWidget.AddToPlayerScreen` _returnvalue_2 0))
    (:`Phase_3`
      (bind _returnvalue_3 (`|CreateWidget` "/Game/Racketeers/Blueprints/Widgets/PhaseWidgets/WBP_Phase3StatsScreen.WBP_Phase3StatsScreen_C" (`GameplayStatics.GetPlayerController` 0)))
      (`UserWidget.AddToPlayerScreen` _returnvalue_3 0))))

(fn `UserConstructionScript`)
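; Base game state for Racketeers that sets up the HUD and music for the current game phase.
; BeginPlay binds round-finished to show a STOP widget and starts two looping one-second timers.
; AddWidgetToScreen clears its timer, updates living teams, then adds phase-specific widgets and triggers music through the game instance, treating NONE as Phase 1.
; CheckPlayersJoinedIn stops polling once expected players join; its retry limit does nothing.
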(event `CheckPlayersJoinedIn`
  (if (== (`KismetArrayLibrary.Array_Length` (`self.PlayerArray`)) (`self.ExpectedPlayers`))
    (`KismetSystemLibrary.K2_ClearAndInvalidateTimerHandle` (`self.CacheHandlePlayerJoined`))
    (else
      (bind _result (`/Engine/EditorBlueprintResources/StandardMacros.IncrementInt` (`self.count`))
        (:`  `
          (if (>= _result 10)
            _))))))

(event `OnClientRoundFinished_Event`
  (bind _returnvalue (`|CreateWidget` "/Game/Racketeers/Blueprints/Widgets/PhaseWidgets/WBP_STOP.WBP_STOP_C"))
  (`UserWidget.AddToViewport` _returnvalue 9999))

(event `self.ReceiveBeginPlay`
  (`parent.ReceiveBeginPlay`)
  (add `self.OnClientRoundFinished` (delegate `OnClientRoundFinished_Event`))
  (bind _returnvalue (`KismetSystemLibrary.K2_SetTimerDelegate` (`|CreateDelegate` :!event `AddWidgetToScreen`) 1.0 true))
  (set `self.Cache Handle` _returnvalue)
  (bind _returnvalue_2 (`KismetSystemLibrary.K2_SetTimerDelegate` (`|CreateDelegate` :!event `CheckPlayersJoinedIn`) 1.0 true))
  (set `self.CacheHandlePlayerJoined` _returnvalue_2))

(event `AddWidgetToScreen`
  (`KismetSystemLibrary.K2_ClearAndInvalidateTimerHandle` (`self.Cache Handle`))
  (`self.UpdateTeamAlive`)
  (switch `EPhaseState` (`self.CurrentPhase`)
    (:`Phase_1`
      (bind _returnvalue (`|CreateWidget` "/Game/Racketeers/Blueprints/Widgets/PlayAndBoat/WBP_TeamResources.WBP_TeamResources_C" :!label _label))
      (`UserWidget.AddToViewport` _returnvalue 0)
      (bind _asbp_base_game_instance (cast `/Game/Racketeers/Core/Framework/BP_BaseGameInstance` (`GameplayStatics.GetGameInstance`)))
      (`/Game/Racketeers/Core/Framework/BP_BaseGameInstance.ActivatePhase1Music` _asbp_base_game_instance))
    (:`Phase_2`
      (bind _asbp_base_game_instance_2 (cast `/Game/Racketeers/Core/Framework/BP_BaseGameInstance` (`GameplayStatics.GetGameInstance`)))
      (`/Game/Racketeers/Core/Framework/BP_BaseGameInstance.ActivatePhase2Music` _asbp_base_game_instance_2))
    (:`Phase_3`
      (bind _returnvalue_2 (`|CreateWidget` "/Game/Racketeers/Blueprints/Widgets/PlayAndBoat/WBP_BoatCount.WBP_BoatCount_C"))
      (`UserWidget.AddToViewport` _returnvalue_2 0)
      (bind _asbp_base_game_instance_3 (cast `/Game/Racketeers/Core/Framework/BP_BaseGameInstance` (`GameplayStatics.GetGameInstance`)))
      (`/Game/Racketeers/Core/Framework/BP_BaseGameInstance.ActivatePhase3Music` _asbp_base_game_instance_3))
    (:`Phase_NONE`
      (goto _label))))

(fn `UserConstructionScript`)
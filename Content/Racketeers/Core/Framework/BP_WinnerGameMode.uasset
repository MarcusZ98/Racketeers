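; Game mode for the winner screen, which places players and team ships by match result and returns to the Lobby once every player has requested it.
; ChoosePlayerStart matches PlayerStart tags built from Winner/Loser and team player ID.
; After a startup delay, collapsed graphs find team players with ID 0, derive boat class, materials and stats from GameState ship parts, then spawn and configure boats at winner/loser spawn tags.
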(event `LoadIntoLobby`
  (`AdvancedSessionsLibrary.ServerTravel` "Lobby"))

(event `self.K2_PostLogin`
  (params (NewPlayer :type "PlayerController Object Reference")))

(event `self.ReceiveTick`
  (params (DeltaSeconds :type "Float (single-precision)")))

(event `self.ReceiveBeginPlay`
  ;[1 1 1] Spawn ships
  ;;[1 1 1] Waiting for players to spawn
  (`KismetSystemLibrary.Delay` 3.0)
  ;;[1 1 1] Searching through Player array
  (bind (_team _teamplayerid) (`self.GetActivePlayers`))
  ;;[1 1 1] Setting Actor to spawn and Spawn position
  (`self.SetAndGetValues` _team _teamplayerid)
  ;;[1 1 1] Spawning the Ship
  (`self.SpawnBoat` (`self.Spawn Pos Actor`) (`self.Spawn Tag`) (`self.Spawn Actor`))
  ;;[1 1 1] Set values for Boat
  (`self.SetValuesBoat`))

(fn `ChoosePlayerStart`
  (params (Player :type "Controller Object Reference"))
  (returns (ReturnValue :type "Actor Object Reference"))
  (locals (TeamStatus :type String))
  (bind _asbp_player_state (cast `/Game/Racketeers/Characters/Blueprints/BP_PlayerState` (`Controller.PlayerState` Player)))
  (bind _asracketeers_game_state_base (cast `RacketeersGameStateBase` (`GameplayStatics.GetGameState`)))
  (bind _gamewinner (`RacketeersGameStateBase.GameWinner` _asracketeers_game_state_base))
  (`KismetSystemLibrary.PrintString` (`KismetStringLibrary.Concat_StrStr` "MAP WINNER " (`|GetEnumeratorNameAsString` _gamewinner)))
  (bind (_playercontroller _playername _bisready _playerstate _team _teamplayerid) (break `PlayerInfo` (`PS_Base.PlayerInfo` _asbp_player_state)))
  (if (== (`KismetSystemLibrary.MakeLiteralByte` _gamewinner) (`KismetSystemLibrary.MakeLiteralByte` _team))
    (set `local.TeamStatus` "Winner")
    (else
      (set `local.TeamStatus` "Loser")))
  (bind _outactors (`GameplayStatics.GetAllActorsOfClass` "/Script/Engine.PlayerStart"))
  (for _array_element _outactors
    (bind _playerstarttag (`PlayerStart.PlayerStartTag` _array_element))
    (bind _returnvalue (`KismetStringLibrary.Concat_StrStr` (`local.TeamStatus`) (`KismetStringLibrary.Conv_IntToString` _teamplayerid)))
    (if (== _playerstarttag (`KismetSystemLibrary.MakeLiteralName` (`KismetStringLibrary.Conv_StringToName` _returnvalue)))
      (return _array_element)
      (else
        (`KismetSystemLibrary.PrintString` (`KismetStringLibrary.Concat_StrStr` (`KismetStringLibrary.Conv_NameToString` _playerstarttag) _returnvalue) true true (struct :`G` 0.66 :`B` 1.0 :`A` 1.0) 7.0))))
  (bind _returnvalue_2 (`parent.ChoosePlayerStart` Player))
  (return _returnvalue_2))

(fn `IncrementLobbyRequestCount`
  (bind _result (`/Engine/EditorBlueprintResources/StandardMacros.IncrementInt` (`self.GoToLobbyCount`))
    (:`  `
      (if (== _result (`KismetArrayLibrary.Array_Length` (`GameStateBase.PlayerArray` (`GameplayStatics.GetGameState`))))
        (`self.LoadIntoLobby`)
        (set `self.GoToLobbyCount` 0)
        (return)))))

(fn `UserConstructionScript`)
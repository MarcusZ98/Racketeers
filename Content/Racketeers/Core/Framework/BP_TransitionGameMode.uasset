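; Game mode for the transition stage between levels and phases in Racketeers.
; On BeginPlay it reads the game mode data from BP_BaseGameInstance, taking the level to load and the phase.
; It passes that phase to BP_TransitionGameState as the incoming phase and prints debug messages, but does no level loading itself.
; On EndPlay it removes all widgets.
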(event `self.K2_PostLogin`
  (params (NewPlayer :type "PlayerController Object Reference")))

(event `self.ReceiveBeginPlay`
  (`KismetSystemLibrary.PrintString` "Begin Play Transition Game Mode")
  (bind _asbp_base_game_instance (cast `/Game/Racketeers/Core/Framework/BP_BaseGameInstance` (`GameplayStatics.GetGameInstance`))
    (:`then`
      (bind _returnvalue (`BaseGameInstance.GetGameModeData` _asbp_base_game_instance))
      (bind _output_get (set `self.LevelToLoad` (break `GameModeData` _returnvalue)))
      (bind _output_get_2 (set `self.State` (`.Phase` (break `GameModeData` _returnvalue))))
      (bind _asbp_transition_game_state (cast `/Game/Racketeers/Core/Framework/BP_TransitionGameState` (`GameplayStatics.GetGameState`)))
      (set `RacketeersGameStateBase.IncomingPhase` _output_get_2 _asbp_transition_game_state)
      (`KismetSystemLibrary.PrintString` _output_get))
    (:`CastFailed`
      (`KismetSystemLibrary.PrintString` "Cast failed Transition Game Mode, in  Base Game Instance" true true (struct :`G` 0.66 :`B` 1.0 :`A` 1.0) 10.0))))

(event `self.ReceiveEndPlay`
  (params (EndPlayReason :type "EEndPlayReason Enum" :default "Destroyed"))
  (`WidgetLayoutLibrary.RemoveAllWidgets`))

(event `self.ReceiveTick`
  (params (DeltaSeconds :type "Float (single-precision)")))

(fn `UserConstructionScript`)
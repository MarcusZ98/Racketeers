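; BP_WinnerGameState is a game state Blueprint for displaying the winner screen in Racketeers.
; BeginPlay starts a looping one-second timer and stores its handle.
; A custom AddWidgettoScreen event, apparently the timer's callback, clears a timer handle, then creates WBP_WinnerWidget and adds it to the viewport.
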(event `self.ReceiveBeginPlay`
  (`parent.ReceiveBeginPlay`)
  (bind _returnvalue (`KismetSystemLibrary.K2_SetTimerDelegate` (`|CreateDelegate` :!event `AddWidgetToScreen`) 1.0 true))
  (set `self.NewVar` _returnvalue))

(event `self.AddWidgetToScreen`
  (`KismetSystemLibrary.K2_ClearAndInvalidateTimerHandle` (`self.Cache Handle`))
  (bind _returnvalue (`|CreateWidget` "/Game/Racketeers/Blueprints/Widgets/WBP_WinnerWidget.WBP_WinnerWidget_C"))
  (`UserWidget.AddToViewport` _returnvalue 0))

(fn `UserConstructionScript`
  (`parent.UserConstructionScript`))
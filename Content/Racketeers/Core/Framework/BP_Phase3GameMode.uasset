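; Phase 3 game mode for Racketeers that spawns and configures a team ship after a short BeginPlay delay for players to join.
; It reads team and slot from the first PlayerArray entry only, as the lookup loop returns immediately, so one boat spawns.
; The team's GameState hull, cannon and sail tiers set boat class, health, cannon count and movement.
; The boat spawns at a team-and-slot tagged actor, then receives those values and team materials.
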(event `self.ReceiveBeginPlay`
  ;[1 1 1] Spawn ships
  ;;[1 1 1] Waiting for players to spawn
  (`KismetSystemLibrary.Delay` 3.0)
  ;;[1 1 1] Searching through Player array
  (bind (_team _teamplayerid) (`self.GetActivePlayers`))
  ;;[1 1 1] Setting Actor to spawn and Spawn position
  (`self.SetAndGetValues` _team _teamplayerid)
  ;;[1 1 1] Spawning the Ship
  (`self.SpawnBoat` (`self.Spawn Pos Actor`) (`self.Spawn Tag`) (`self.Spawn Actor`))
  ;;[1 1 1] Set values for Boat
  (`self.SetValuesBoat`))

(fn `GetPlayerStartPosf`
  (params (Tag :type Name))
  (returns (Location :type "Vector Structure"))
  (bind _outactors (`GameplayStatics.GetAllActorsOfClassWithTag` "/Script/Engine.PlayerStart" Tag))
  (for _array_element _outactors
    (return (`self.K2_GetActorLocation` _array_element))))

(fn `UserConstructionScript`)
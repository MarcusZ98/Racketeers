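; Base game mode for Racketeers that picks each player's raccoon or red panda pawn and team-tagged start, and spawns team boats.
; After a map loads in the boat phase, it walks the PlayerArray and spawns boats at tagged BP_BoatStartPos actors.
; The team's construction parts in the GameState set boat class, health, cannons, sails and movement.
; Computed rotation speed never reaches the boat, as SetMovement receives zero.
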(event `self.K2_OnSwapPlayerControllers`
  (params (OldPC :type "PlayerController Object Reference") (NewPC :type "PlayerController Object Reference"))
  ;[1 1 1] Triggers when players spawn in the new level
  (add `self.OnloadedMap` (delegate `Spawn ship`)))

(event `Spawn ship`
  ;[1 1 1] Triggers when players spawn in the new level
  ;;[1 1 1] Only run when in Phase 3
  (if (== (`Phase.State` (`self.CurrentPhase`)) 1)
    (`self.SpawnShips`)))

(event `SpawnShips`
  ;[1 1 1] Spawn ships
  ;;[1 1 1] Waiting for players to spawn
  (`KismetSystemLibrary.Delay` 0.2)
  ;;[1 1 1] Searching through Player array
  (bind (_team _teamplayerid) (`self.GetActivePlayers`))
  ;;[1 1 1] Setting Actor to spawn and Spawn position
  (`self.SetAndGetValues` _team _teamplayerid)
  ;;[1 1 1] Spawning the Ship
  (`self.SpawnBoat` "/Game/Developers/jahj7676/Jacob/BP_BoatStartPos.BP_BoatStartPos_C" (`self.Spawn Tag`) (`self.Spawn Actor`))
  ;;[1 1 1] Set values for Boat
  (`self.SetValuesBoat`))

(event `self.ReceiveBeginPlay`
  (`parent.ReceiveBeginPlay`)
  (`KismetSystemLibrary.PrintString` "BaseGameMode::BegnPLay"))

(fn `ChoosePlayerStart`
  (params (Player :type "Controller Object Reference"))
  (returns (ReturnValue :type "Actor Object Reference"))
  (bind _asbp_player_state (cast `/Game/Racketeers/Characters/Blueprints/BP_PlayerState` (`Controller.PlayerState` Player)))
  (bind _outactors (`GameplayStatics.GetAllActorsOfClass` "/Script/Engine.PlayerStart"))
  (for _array_element _outactors
    (bind (_playercontroller _playername _bisready _playerstate _team _teamplayerid) (break `PlayerInfo` (`PS_Base.PlayerInfo` _asbp_player_state)))
    (if (== (`PlayerStart.PlayerStartTag` _array_element) (`KismetSystemLibrary.MakeLiteralName` (`KismetStringLibrary.Conv_StringToName` (`KismetStringLibrary.Concat_StrStr` (`|GetEnumeratorNameAsString` _team) (`KismetStringLibrary.Conv_IntToString` _teamplayerid)))))
      (return _array_element)))
  (bind _returnvalue (`parent.ChoosePlayerStart` null))
  (return _returnvalue))

(fn `GetDefaultPawnClassForController`
  (params (InController :type "Controller Object Reference"))
  (returns (ReturnValue :type "Object Class Reference"))
  (bind _asbp_player_state (cast `/Game/Racketeers/Characters/Blueprints/BP_PlayerState` (`Controller.PlayerState` InController)))
  (bind (_playerinfo_playercontroller _playerinfo_playername _playerinfo_bisready _playerinfo_playerstate _playerinfo_team) (break `PlayerInfo` (`PS_Base.PlayerInfo` _asbp_player_state)))
  (bind _returnvalue (select `ETeams` _playerinfo_team :`Team_Raccoon` "/Game/Racketeers/Characters/Blueprints/BP_Racoon.BP_Racoon_C" :`Team_Panda` "/Game/Racketeers/Characters/Blueprints/BP_RedPanda.BP_RedPanda_C" :`NONE` "/Game/Racketeers/Characters/Blueprints/BP_Racoon.BP_Racoon_C" :!type "Object Class Reference"))
  (if (`KismetSystemLibrary.IsValidClass` _returnvalue)
    (return _returnvalue)
    (else
      (return "/Game/Racketeers/Core/BP_Player.BP_Player_C"))))

(fn `GetPlayerStartPos`
  (params (Tag :type Name))
  (returns (Location :type "Vector Structure"))
  (bind _outactors (`GameplayStatics.GetAllActorsOfClassWithTag` "/Script/Engine.PlayerStart" Tag))
  (for _array_element _outactors
    (return (`self.K2_GetActorLocation` _array_element))))

(fn `LookForPlayers`
  (returns (Team :type "ETeams Enum") (TeamPlayerID :type Integer))
  (bind (_team _teamplayerid) (`self.GetActivePlayers`))
  (return _team _teamplayerid))

(fn `UserConstructionScript`)
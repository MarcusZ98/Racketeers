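; BP_Player_Boat is an interactable boat pawn that a player takes control of by interacting with it.
; StartInteract forwards the instigator to Server_StartInteract2, which casts its controller to BP_PlayerController, checks for a BP_PlayerState, then has that controller possess the boat.
; CanInteract always returns true, the separate ServerStartInteract function is an empty stub, and the file holds no movement or exit logic.
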(event `self.StartInteract`
  (params (Instigator :type "Actor Object Reference") (bIsServer :type Boolean))
  (`self.Server_StartInteract2` Instigator))

(event `Server_StartInteract2`
  (params (Instigator :type "Actor Object Reference"))
  (bind _asbp_player_controller (cast `/Game/Racketeers/Characters/Blueprints/PCs/BP_PlayerController` (`self.GetInstigatorController` Instigator)))
  (cast `/Game/Racketeers/Characters/Blueprints/BP_PlayerState` (`Controller.PlayerState` _asbp_player_controller))
  (`Controller.Possess` _asbp_player_controller self))

(fn `CanInteract`
  (returns (ReturnValue :type Boolean))
  (return true))

(fn `Server_StartInteract`
  (params (Instigator1 :type "Actor Object Reference")))

(fn `UserConstructionScript`
  (`parent.UserConstructionScript`))
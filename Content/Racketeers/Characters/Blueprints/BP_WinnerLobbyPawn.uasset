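; BP_WinnerLobbyPawn is the player pawn for the post-match winner screen, letting players request a return to the lobby or leave the game.
; It adds the winner widget to the viewport on BeginPlay.
; Interact sends a one-time lobby request, which increments the request count on BP_WinnerGameMode.
; Jump exits: the server returns the host to the main menu, while a client calls KickPlayer on its controller.
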(event `GoToLobbyRequested`
  (bind _asbp_winner_game_mode (cast `/Game/Racketeers/Core/Framework/BP_WinnerGameMode` (`GameplayStatics.GetGameMode`)))
  (`/Game/Racketeers/Core/Framework/BP_WinnerGameMode.IncrementLobbyRequestCount` _asbp_winner_game_mode))

(event `self.ReceiveBeginPlay`
  (`UserWidget.AddToViewport` (`self.WinnerWidget`) 0))

(event `EnhancedInput|/Game/Racketeers/Characters/Input/Actions/IA_Interact`
  (params (ActionValue :type Boolean) (ElapsedSeconds :type "Float (double-precision)") (TriggeredSeconds :type "Float (double-precision)") (InputAction :type "InputAction Object Reference" :default "/Game/Racketeers/Characters/Input/Actions/IA_Interact.IA_Interact"))
  (:`Started`
    (if (not (`self.Pressed Continue`))
      (`self.GoToLobbyRequested`)
      (set `self.Pressed Continue` true))))

(event `EnhancedInput|/Game/Racketeers/Characters/Input/Actions/IA_Jump`
  (params (ActionValue :type Boolean) (ElapsedSeconds :type "Float (double-precision)") (TriggeredSeconds :type "Float (double-precision)") (InputAction :type "InputAction Object Reference" :default "/Game/Racketeers/Characters/Input/Actions/IA_Jump.IA_Jump"))
  (:`Started`
    (`self.GoToMainMenu` (`GameplayStatics.GetPlayerController` 0) (`KismetSystemLibrary.IsServer`))))

(event `GoToMainMenu`
  (params (PC :type "PlayerController Object Reference") (IsServer :type Boolean))
  (if IsServer
    (`GameModeBase.ReturnToMainMenuHost` (`GameplayStatics.GetGameMode`))
    (else
      (`AdvancedSessionsLibrary.KickPlayer` PC))))

(fn `UserConstructionScript`)
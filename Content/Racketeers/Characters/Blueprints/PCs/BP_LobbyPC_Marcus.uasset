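; Lobby player controller that plays iris screen transitions when the lobby opens and when the match starts.
; On BeginPlay, after the parent logic, it creates a WBP_Transition widget, plays its iris-in and removes it after a short fixed delay.
; OnStartMatch creates a fresh transition widget, plays the iris-out and disables the player's input, leaving the widget on screen.
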(event `self.ReceiveBeginPlay`
  (`parent.ReceiveBeginPlay`)
  (bind _returnvalue (`|CreateWidget` "/Game/Racketeers/Blueprints/Widgets/WBP_Transition.WBP_Transition_C" self))
  (`UserWidget.AddToViewport` _returnvalue 0)
  (`/Game/Racketeers/Blueprints/Widgets/WBP_Transition.IrisIn` _returnvalue)
  (`KismetSystemLibrary.Delay` 1.0)
  (`Widget.RemoveFromParent` _returnvalue))

(event `self.OnStartMatch`
  (bind _returnvalue (`|CreateWidget` "/Game/Racketeers/Blueprints/Widgets/WBP_Transition.WBP_Transition_C" self))
  (`UserWidget.AddToViewport` _returnvalue 0)
  (`/Game/Racketeers/Blueprints/Widgets/WBP_Transition.IrisOut` _returnvalue)
  (`self.DisableInput` self))

(fn `UserConstructionScript`)